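; FightUnitUniversal is a character Blueprint for a fight unit that modulates its walk speed during movement.
; On BeginPlay it reads the base speed from an Ability System attribute after a short delay.
; Each tick scales MaxWalkSpeed by a landing factor, zeroed while falling and ramping up over LandingTime, and a cubed penalty for input angled away from facing.
; An arrow is shown and MovementInput is rotated to the last input direction.
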(event `self.ReceiveBeginPlay`
  (`SceneComponent.SetHiddenInGame` (`self.ArrowComponent`) false false)
  (`KismetSystemLibrary.Delay` 0.2)
  (`self.GetWalkSpeed`)
  (set `self.LandingTimeStamp` (- (`self.GetGameTimeSinceCreation`) (`self.LandingTime`))))

(event `self.ReceiveTick`
  (params (DeltaSeconds :type "Float (single-precision)"))
  (`SceneComponent.K2_SetWorldRotation` (`self.MovementInput`) (`KismetMathLibrary.Conv_VectorToRotator` (`self.GetLastMovementInputVector`)) false false)
  (`self.UpdateFallingPhysics`)
  (`self.CalculateRotationFactor`)
  (set `CharacterMovementComponent.MaxWalkSpeed` (* (`self.WalkSpeed`) (`self.LandingFactor`) (`KismetMathLibrary.MultiplyMultiply_FloatFloat` (- 1.0 (`self.RotationFactor`)) 3.0)) (`self.CharacterMovement`)))

(fn `CalculateRotationFactor`
  (set `self.RotationFactor` (`KismetMathLibrary.SelectFloat` 0.0 (`KismetMathLibrary.MapRangeClamped` (`KismetMathLibrary.Abs` (`self.NormalizeDegree180180` (`self.AngleDiffVec` (`self.GetLastMovementInputVector`) (`self.GetActorForwardVector`)))) 0.0 180.0 0.0 0.4) (< (`KismetMathLibrary.VSize` (`self.GetLastMovementInputVector`)) 0.1))))

(fn `GetWalkSpeed`
  (bind _abilitysystem (`self.AbilitySystem`))
  (bind (_bsuccessfullyfoundattribute _returnvalue) (`AbilitySystemBlueprintLibrary.GetFloatAttributeFromAbilitySystemComponent` _abilitysystem (struct :`AttributeName` "MoveSpeed" :`Attribute` "/Script/LinhiBlade.AP_AttributeSet:MoveSpeed")))
  (`/Engine/EditorBlueprintResources/StandardMacros.IsValid` _abilitysystem
    (:`Is Valid`
      (if _bsuccessfullyfoundattribute
        (set `self.WalkSpeed` _returnvalue)
        (return)
        (else
          (`KismetSystemLibrary.PrintString` "GetWalkSpeed called too early, no Attribute found")
          (return))))
    (:`Is Not Valid`
      (`KismetSystemLibrary.PrintString` "GetWalkSpeed called too early, no AbilitySystem found")
      (return))))

(fn `UpdateFallingPhysics`
  (locals (TimeSinceLanding :type "Float (double-precision)" :default 0.0))
  (if (`NavMovementComponent.IsFalling` (`self.CharacterMovement`))
    (set `self.LandingFactor` 0.0)
    (set `self.IsFallingLastFrame` true)
    (return)
    (else
      (if (`self.IsFallingLastFrame`)
        (set `self.LandingTimeStamp` (`self.GetGameTimeSinceCreation`)))
      (bind _output_get (set `local.TimeSinceLanding` (- (`self.GetGameTimeSinceCreation`) (`self.LandingTimeStamp`))))
      (set `self.LandingFactor` (`KismetMathLibrary.FClamp` (/ _output_get (`self.LandingTime`))))
      (set `self.IsFallingLastFrame` (`NavMovementComponent.IsFalling` (`self.CharacterMovement`)))
      (return))))

(fn `UserConstructionScript`)
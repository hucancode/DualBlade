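; Axe_In_World is a timed world axe tied to a buff on the Female_Hero's ability system.
; Tick lerps the axe component's relative location from an original point to a destination over a falling time, then holds it there.
; BeginPlay sets the actor's lifespan.
; On destruction, RemoveBuff strips active effects matching the buff class's granted tags and calls SetupWeapon on the owning hero to switch weapon setup.
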(event `self.ReceiveBeginPlay`
  (`self.SetLifeSpan` (`self.Lifespan`)))

(event `self.ReceiveTick`
  (params (DeltaSeconds :type "Float (single-precision)"))
  (`SceneComponent.K2_SetRelativeLocation` (`self.Axe`) (`KismetMathLibrary.VLerp` (`self.Original`) (`self.Destination`) (`KismetMathLibrary.FMin` (/ (`self.GetGameTimeSinceCreation`) (`self.Falling_Time`)) 1.0)) false false))

(event `self.ReceiveDestroyed`
  (`self.RemoveBuff`))

(fn `RemoveBuff`
  (bind _parentabilitysystem (`self.ParentAbilitySystem`))
  (`AbilitySystemComponent.RemoveActiveEffectsWithGrantedTags` _parentabilitysystem (`.CombinedTags` (break `InheritedTagContainer` (`.InheritableOwnedTagsContainer` (defaults `/Game/AgeOfDualBlade/Blueprints/Axe_In_World` (`self.Buff_Class`))))))
  (bind _asfemale_hero (cast `/Game/AgeOfDualBlade/Blueprints/Female_Hero` (`ActorComponent.GetOwner` _parentabilitysystem)))
  (`/Game/AgeOfDualBlade/Blueprints/Female_Hero.SetupWeapon` _asfemale_hero "NewEnumerator1"))

(fn `UserConstructionScript`)
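; Falling arrow actor, likely a single projectile of an Arrow Field ability, that damages heroes it touches and expires after its lifespan.
; Each tick it lerps its height from the spawn Z down to world Z zero over the falling time, guarding against a zero duration.
; When its capsule overlaps an AP_Hero, the parent ability system, if valid, applies the damage GameplayEffect to that hero.
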(event `self.ReceiveBeginPlay`
  (`self.SetLifeSpan` (`self.Lifespan`))
  (set `self.Original_Z` (.z (`self.K2_GetActorLocation`))))

(event `self.ReceiveTick`
  (params (DeltaSeconds :type "Float (single-precision)"))
  (bind _fallingtime (`self.FallingTime`))
  (`self.K2_SetActorLocation` (`KismetMathLibrary.MakeVector` (.x (`self.K2_GetActorLocation`)) (.y (`self.K2_GetActorLocation`)) (`KismetMathLibrary.Lerp` (`self.Original_Z`) 0.0 (`KismetMathLibrary.FClamp` (/ (`self.GetGameTimeSinceCreation`) (`KismetMathLibrary.SelectFloat` 1.0 _fallingtime (`KismetMathLibrary.NearlyEqual_FloatFloat` _fallingtime))))))))

(event `self.Capsule.OnComponentBeginOverlap`
  (params (OverlappedComponent :type "PrimitiveComponent Object Reference") (OtherActor :type "Actor Object Reference") (OtherComp :type "PrimitiveComponent Object Reference") (OtherBodyIndex :type Integer) (bFromSweep :type Boolean) (SweepResult :type "HitResult Structure (by ref)"))
  (bind _parentabilitysystem (`self.ParentAbilitySystem`))
  (bind _asap_hero (cast `AP_Hero` OtherActor))
  (`/Engine/EditorBlueprintResources/StandardMacros.IsValid` _parentabilitysystem
    (:`Is Valid`
      (`AbilitySystemComponent.BP_ApplyGameplayEffectToTarget` :`self` _parentabilitysystem :`GameplayEffectClass` (`self.DamageClass`) :`Target` (`AbilitySystemBlueprintLibrary.GetAbilitySystemComponent` _asap_hero) :`Level` 1.0))))

(fn `UserConstructionScript`)
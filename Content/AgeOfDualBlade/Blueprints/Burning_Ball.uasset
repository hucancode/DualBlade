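; Burning_Ball is a timed area actor that puts a gameplay effect on heroes while they are inside its sphere.
; On overlap begin, an AP_Hero receives DamageBuffClass from ParentAbilitySystem through the Gameplay Ability System.
; On overlap end, all stacks of that effect are removed from the hero, with no instigator filter.
; Despite the variable name, debug prints call the effect a silence.
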(event `self.ReceiveBeginPlay`
  (`self.SetLifeSpan` (`self.Lifespan`)))

(event `self.Sphere.OnComponentBeginOverlap`
  (params (OverlappedComponent :type "PrimitiveComponent Object Reference") (OtherActor :type "Actor Object Reference") (OtherComp :type "PrimitiveComponent Object Reference") (OtherBodyIndex :type Integer) (bFromSweep :type Boolean) (SweepResult :type "HitResult Structure (by ref)"))
  (bind _asap_hero (cast `AP_Hero` OtherActor))
  (`self.ApplyBuff` _asap_hero))

(event `self.Sphere.OnComponentEndOverlap`
  (params (OverlappedComponent :type "PrimitiveComponent Object Reference") (OtherActor :type "Actor Object Reference") (OtherComp :type "PrimitiveComponent Object Reference") (OtherBodyIndex :type Integer))
  (bind _asap_hero (cast `AP_Hero` OtherActor))
  (`self.RemoveBuff` _asap_hero))

(fn `ApplyBuff`
  (params (Target :type "AP_Hero Object Reference"))
  (`AbilitySystemComponent.BP_ApplyGameplayEffectToTarget` :`self` (`self.ParentAbilitySystem`) :`GameplayEffectClass` (`self.Damage_Buff_Class`) :`Target` (`AbilitySystemBlueprintLibrary.GetAbilitySystemComponent` Target))
  (`KismetSystemLibrary.PrintString` "apply silence"))

(fn `RemoveBuff`
  (params (Target :type "AP_Hero Object Reference"))
  (`AbilitySystemComponent.RemoveActiveGameplayEffectBySourceEffect` (`AbilitySystemBlueprintLibrary.GetAbilitySystemComponent` Target) (`self.Damage_Buff_Class`) null -1)
  (`KismetSystemLibrary.PrintString` "remove silence buff"))

(fn `UserConstructionScript`)
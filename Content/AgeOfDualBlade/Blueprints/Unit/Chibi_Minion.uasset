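; Chibi minion unit Blueprint that shows floating health and mana bars and can vanish and reappear.
; BeginPlay fills both bars, and health and mana change events push current percentages to the FloatingResourceBar widget, with a debug print on health changes.
; Vanish start hides and deactivates capsule, selection box and movement; finish reactivates them and restores mesh, bar and selection ring, the ring only if selected.
; Disconnected setup logic for controller spawning and selection component placement never runs.
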(event `self.OnHealthChanged`
  (params (NewValue :type "Float (single-precision)"))
  (`KismetSystemLibrary.PrintString` (`KismetStringLibrary.Concat_StrStr` "hit, damage = " (`KismetStringLibrary.Conv_DoubleToString` 0.0)))
  (bind _asfloating_resource_bar (cast `/Game/Common/FloatingResourceBar` (`WidgetComponent.GetUserWidgetObject` (`self.ResourceBar`))))
  (`/Game/Common/FloatingResourceBar.SetHPPercent` _asfloating_resource_bar (`self.GetHealthPercent`)))

(event `self.OnManaChanged`
  (params (NewValue :type "Float (single-precision)"))
  (bind _asfloating_resource_bar (cast `/Game/Common/FloatingResourceBar` (`WidgetComponent.GetUserWidgetObject` (`self.ResourceBar`))))
  (`/Game/Common/FloatingResourceBar.SetMPPercent` _asfloating_resource_bar (`self.GetManaPercent`)))

(event `self.ReceiveBeginPlay`
  (bind _asfloating_resource_bar (cast `/Game/Common/FloatingResourceBar` (`WidgetComponent.GetUserWidgetObject` (`self.ResourceBar`))))
  (`/Game/Common/FloatingResourceBar.SetHPPercent` _asfloating_resource_bar 1.0)
  (`/Game/Common/FloatingResourceBar.SetMPPercent` _asfloating_resource_bar 1.0))

(event `self.OnVanishedStarted`
  (`SceneComponent.SetVisibility` (`self.CapsuleComponent`) false true)
  (`ActorComponent.Deactivate` (`self.CapsuleComponent`))
  (`ActorComponent.Deactivate` (`self.SelectionBox`))
  (`ActorComponent.Deactivate` (`self.CharacterMovement`)))

(event `self.OnVanishedFinished`
  (`ActorComponent.Activate` (`self.CapsuleComponent`) false)
  (`ActorComponent.Activate` (`self.SelectionBox`) false)
  (`ActorComponent.Activate` (`self.CharacterMovement`) false)
  (`SceneComponent.SetVisibility` (`self.ResourceBar`) true false)
  (`SceneComponent.SetVisibility` (`self.Mesh`) true false)
  (`SceneComponent.SetVisibility` (`self.SelectionRing`) (`self.IsSelected`) false))

(fn `UserConstructionScript`)
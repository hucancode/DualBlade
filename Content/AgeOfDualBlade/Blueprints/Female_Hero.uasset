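; Female hero character with modular body and weapon meshes on a master pose, a floating HP/MP bar and switchable weapons.
; SetupWeapon swaps visible meshes and, when the normalized weapon family changes, replaces the ability set and plays any intro montage.
; Overlapping a TriggerSphere cycles weapons, recursively skipping variant states.
; Vanish events hide and deactivate capsule, selection box and movement, then restore them with the current weapon.
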(event `self.OnHealthChanged`
  (params (NewValue :type "Float (single-precision)"))
  (`KismetSystemLibrary.PrintString` (`KismetStringLibrary.Concat_StrStr` "hit, damage = " (`KismetStringLibrary.Conv_DoubleToString` 0.0)))
  (bind _asfloating_resource_bar (cast `/Game/Common/FloatingResourceBar` (`WidgetComponent.GetUserWidgetObject` (`self.ResourceBar`))))
  (`/Game/Common/FloatingResourceBar.SetHPPercent` _asfloating_resource_bar (/ (`self.GetHealth`) (`self.GetMaxHealth`))))

(event `self.OnManaChanged`
  (params (NewValue :type "Float (single-precision)"))
  (bind _asfloating_resource_bar (cast `/Game/Common/FloatingResourceBar` (`WidgetComponent.GetUserWidgetObject` (`self.ResourceBar`))))
  (`/Game/Common/FloatingResourceBar.SetMPPercent` _asfloating_resource_bar (/ (`self.GetMana`) (`self.GetMaxMana`))))

(event `self.ReceiveBeginPlay`
  (bind _asfloating_resource_bar (cast `/Game/Common/FloatingResourceBar` (`WidgetComponent.GetUserWidgetObject` (`self.ResourceBar`))))
  (`/Game/Common/FloatingResourceBar.SetHPPercent` _asfloating_resource_bar 1.0)
  (`/Game/Common/FloatingResourceBar.SetMPPercent` _asfloating_resource_bar 1.0)
  (`SkinnedMeshComponent.SetLeaderPoseComponent` (`self.Dual_Sword`) (`self.Mesh`) false)
  (`SkinnedMeshComponent.SetLeaderPoseComponent` (`self.Body_Upper`) (`self.Mesh`) false)
  (`SkinnedMeshComponent.SetLeaderPoseComponent` (`self.Head`) (`self.Mesh`) false)
  (`SkinnedMeshComponent.SetLeaderPoseComponent` (`self.Body_Lower`) (`self.Mesh`) false)
  (`SkinnedMeshComponent.SetLeaderPoseComponent` (`self.Hair`) (`self.Mesh`) false)
  (`SkinnedMeshComponent.SetLeaderPoseComponent` (`self.Hand_L`) (`self.Mesh`) false)
  (`SkinnedMeshComponent.SetLeaderPoseComponent` (`self.Claw`) (`self.Mesh`) false)
  (`SkinnedMeshComponent.SetLeaderPoseComponent` (`self.Feet`) (`self.Mesh`) false)
  (`SkinnedMeshComponent.SetLeaderPoseComponent` (`self.Bow`) (`self.Mesh`) false)
  (`SkinnedMeshComponent.SetLeaderPoseComponent` (`self.Axe`) (`self.Mesh`) false)
  (`SkinnedMeshComponent.SetLeaderPoseComponent` (`self.Katana`) (`self.Mesh`) false)
  (`SkinnedMeshComponent.SetLeaderPoseComponent` (`self.Magic_Staff`) (`self.Mesh`) false)
  (`SkinnedMeshComponent.SetLeaderPoseComponent` (`self.Sword_Shield`) (`self.Mesh`) false)
  (`SkinnedMeshComponent.SetLeaderPoseComponent` (`self.Dagger`) (`self.Mesh`) false)
  (`SkinnedMeshComponent.SetLeaderPoseComponent` (`self.Sword_R`) (`self.Mesh`) false)
  (`self.SetupWeapon` (`self.CurrentWeapon`)))

(event `self.CapsuleComponent.OnComponentBeginOverlap`
  (params (OverlappedComponent :type "PrimitiveComponent Object Reference") (OtherActor :type "Actor Object Reference") (OtherComp :type "PrimitiveComponent Object Reference") (OtherBodyIndex :type Integer) (bFromSweep :type Boolean) (SweepResult :type "HitResult Structure (by ref)"))
  (if (== (`GameplayStatics.GetObjectClass` OtherActor) "/Script/Engine.TriggerSphere")
    (`self.CycleWeapon` 1)))

(event `self.OnVanishedStarted`
  (`SceneComponent.SetVisibility` (`self.CapsuleComponent`) false true)
  (`ActorComponent.Deactivate` (`self.CapsuleComponent`))
  (`ActorComponent.Deactivate` (`self.SelectionBox`))
  (`ActorComponent.Deactivate` (`self.CharacterMovement`)))

(event `self.OnVanishedFinished`
  (`ActorComponent.Activate` (`self.CapsuleComponent`) false)
  (`ActorComponent.Activate` (`self.SelectionBox`) false)
  (`ActorComponent.Activate` (`self.CharacterMovement`) false)
  (`SceneComponent.SetVisibility` (`self.ResourceBar`) true false)
  (`SceneComponent.SetVisibility` (`self.Feet`) true false)
  (`SceneComponent.SetVisibility` (`self.Body_Upper`) true false)
  (`SceneComponent.SetVisibility` (`self.Body_Lower`) true false)
  (`SceneComponent.SetVisibility` (`self.Head`) true false)
  (`SceneComponent.SetVisibility` (`self.Hair`) true false)
  (`SceneComponent.SetVisibility` (`self.Hand_L`) true false)
  (`SceneComponent.SetVisibility` (`self.Hand_R`) true false)
  (bind _mesh (`self.GetWeaponMesh` (`self.CurrentWeapon`)))
  (`/Engine/EditorBlueprintResources/StandardMacros.IsValid` _mesh
    (:`Is Valid`
      (`SceneComponent.SetVisibility` _mesh true false)
      (`SceneComponent.SetVisibility` (`self.SelectionRing`) (`self.IsSelected`) false))))

(fn `CycleWeapon`
  (params (Delta :type Integer :default 1))
  (bind _delta (`local.Delta`))
  (bind _returnvalue (cast `/Game/AgeOfDualBlade/Proxy_Meshes/WeaponType` (mod (+ (`self.CurrentWeapon`) (`KismetMathLibrary.Conv_IntToByte` (`local.Delta`))) (`KismetMathLibrary.Conv_IntToByte` (enumcount `/Game/AgeOfDualBlade/Proxy_Meshes/WeaponType`)))))
  (switch `/Game/AgeOfDualBlade/Proxy_Meshes/WeaponType` _returnvalue
    (:`NewEnumerator1`
      (`self.SetupWeapon` _returnvalue :!label _label)
      (return))
    (:`NewEnumerator11`
      _)
    (:`NewEnumerator0`
      (goto _label))
    (:`NewEnumerator2`
      (goto _label))
    (:`NewEnumerator3`
      (goto _label))
    (:`NewEnumerator4`
      (goto _label))
    (:`NewEnumerator5`
      (goto _label))
    (:`NewEnumerator9`
      _)
    (:`NewEnumerator10`
      _)
    (:`NewEnumerator6`
      (goto _label))
    (:`NewEnumerator7`
      (goto _label))
    (:`NewEnumerator12`
      _)
    (:`NewEnumerator13`
      _))
  (`self.CycleWeapon` (* (`KismetMathLibrary.SignOfInteger` _delta) (+ (`KismetMathLibrary.Abs_Int` _delta) 1))))

(fn `GetWeaponMesh`
  (params (Weapon :type "/Game/AgeOfDualBlade/Proxy_Meshes/WeaponType Enum" :default "NewEnumerator1"))
  (returns (Mesh :type "SkeletalMeshComponent Object Reference"))
  (switch `/Game/AgeOfDualBlade/Proxy_Meshes/WeaponType` Weapon
    (:`NewEnumerator1`
      (return (`self.Axe`)))
    (:`NewEnumerator11`
      _)
    (:`NewEnumerator0`
      (return (`self.Bow`)))
    (:`NewEnumerator2`
      (return (`self.Dagger`)))
    (:`NewEnumerator3`
      (return (`self.Dual_Sword`)))
    (:`NewEnumerator4`
      (return (`self.Claw`)))
    (:`NewEnumerator5`
      (return (`self.Katana`)))
    (:`NewEnumerator9`
      (return (`self.Katana`)))
    (:`NewEnumerator10`
      (return (`self.Katana`)))
    (:`NewEnumerator6`
      (return (`self.Magic_Staff`)))
    (:`NewEnumerator7`
      (return (`self.Sword_Shield`)))
    (:`NewEnumerator12`
      (return (`self.Sword_R`)))
    (:`NewEnumerator13`
      _))
  (return null))

(fn `NormalizeWeapon`
  (params (Input :type "/Game/AgeOfDualBlade/Proxy_Meshes/WeaponType Enum" :default "NewEnumerator1"))
  (returns (Output :type "/Game/AgeOfDualBlade/Proxy_Meshes/WeaponType Enum"))
  (switch `/Game/AgeOfDualBlade/Proxy_Meshes/WeaponType` Input
    (:`NewEnumerator1`
      _)
    (:`NewEnumerator11`
      _)
    (:`NewEnumerator0`
      (return Input))
    (:`NewEnumerator2`
      (return Input))
    (:`NewEnumerator3`
      (return Input))
    (:`NewEnumerator4`
      (return Input))
    (:`NewEnumerator5`
      (return "NewEnumerator5"))
    (:`NewEnumerator9`
      (return "NewEnumerator5"))
    (:`NewEnumerator10`
      (return "NewEnumerator5"))
    (:`NewEnumerator6`
      (return Input))
    (:`NewEnumerator7`
      (return "NewEnumerator7"))
    (:`NewEnumerator12`
      (return "NewEnumerator7"))
    (:`NewEnumerator13`
      (return "NewEnumerator7")))
  (return "NewEnumerator1"))

(fn `SetupWeapon`
  (params (NewWeapon :type "/Game/AgeOfDualBlade/Proxy_Meshes/WeaponType Enum" :default "NewEnumerator1"))
  (bind (_value _returnvalue) (`BlueprintMapLibrary.Map_Find` (`self.Intros`) (`self.CurrentWeapon`)))
  (bind _mesh (`self.GetWeaponMesh` (`self.CurrentWeapon`)))
  (`/Engine/EditorBlueprintResources/StandardMacros.IsValid` _mesh
    (:`Is Valid`
      (`SceneComponent.SetVisibility` _mesh false false))
    (:`Is Not Valid`
      _))
  (bind _mesh_2 (`self.GetWeaponMesh` (`local.NewWeapon`)))
  (`/Engine/EditorBlueprintResources/StandardMacros.IsValid` _mesh_2
    (:`Is Valid`
      (`SceneComponent.SetVisibility` _mesh_2 true false))
    (:`Is Not Valid`
      _))
  (bind _result (`self.ShouldKeepSkillSet` (`self.CurrentWeapon`) (`local.NewWeapon`)))
  (if _result
    (set `self.CurrentWeapon` (`local.NewWeapon`))
    (else
      (bind _output_get (set `self.CurrentWeapon` (`local.NewWeapon`)))
      (switch `/Game/AgeOfDualBlade/Proxy_Meshes/WeaponType` _output_get
        (:`NewEnumerator1`
          (set `self.SpellAbilitySet` "/Game/AgeOfDualBlade/Abilities/SkillSets/Axe_Skill_Set.Axe_Skill_Set" :!label _label))
        (:`NewEnumerator11`
          (goto _label))
        (:`NewEnumerator0`
          (set `self.SpellAbilitySet` "/Game/AgeOfDualBlade/Abilities/SkillSets/Bow_Skill_Set.Bow_Skill_Set"))
        (:`NewEnumerator2`
          (set `self.SpellAbilitySet` "/Game/AgeOfDualBlade/Abilities/SkillSets/Dagger_Skill_Set.Dagger_Skill_Set"))
        (:`NewEnumerator3`
          (set `self.SpellAbilitySet` "/Game/AgeOfDualBlade/Abilities/SkillSets/Dual_Skill_Set.Dual_Skill_Set"))
        (:`NewEnumerator4`
          (set `self.SpellAbilitySet` "/Game/AgeOfDualBlade/Abilities/SkillSets/Claw_Skill_Set.Claw_Skill_Set"))
        (:`NewEnumerator5`
          (set `self.SpellAbilitySet` "/Game/AgeOfDualBlade/Abilities/SkillSets/Katana_Skill_Set.Katana_Skill_Set" :!label _label_2))
        (:`NewEnumerator9`
          (goto _label_2))
        (:`NewEnumerator10`
          (goto _label_2))
        (:`NewEnumerator6`
          (set `self.SpellAbilitySet` "/Game/AgeOfDualBlade/Abilities/SkillSets/MagicStaff_Skill_Set.MagicStaff_Skill_Set"))
        (:`NewEnumerator7`
          (set `self.SpellAbilitySet` "/Game/AgeOfDualBlade/Abilities/SkillSets/Sword_Skill_Set.Sword_Skill_Set" :!label _label_3))
        (:`NewEnumerator12`
          (goto _label_3))
        (:`NewEnumerator13`
          (goto _label_3)))
      (`self.RemoveAllAbilities`)
      (`self.SetupAbilities`)
      (if _returnvalue
        (`self.PlayAnimMontage` _value)))))

(fn `ShouldKeepSkillSet`
  (params (OldWeapon :type "/Game/AgeOfDualBlade/Proxy_Meshes/WeaponType Enum" :default "NewEnumerator1") (NewWeapon :type "/Game/AgeOfDualBlade/Proxy_Meshes/WeaponType Enum" :default "NewEnumerator1"))
  (returns (Result :type Boolean))
  (bind _output (`self.NormalizeWeapon` OldWeapon))
  (bind _output_2 (`self.NormalizeWeapon` NewWeapon))
  (return (`|EnumEquality` _output _output_2)))

(fn `UserConstructionScript`)
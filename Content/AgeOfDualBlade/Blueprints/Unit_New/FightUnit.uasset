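; Combat unit Blueprint that binds stat, death, respawn, fight-style and cloak events to its visuals and movement.
; Health and mana changes feed an overhead resource bar and debug prints.
; Fight style selects the visible weapon mesh, slaved to the body via master pose, and sets rotation and jump rules.
; Death parks the actor high above its spawn point until respawn; Vanished cloak hides the mesh, and cloak end reapplies style.
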(event `self.ReceiveBeginPlay`
  (bind _stats (`self.Stats`))
  (bind _teamagent (`self.TeamAgent`))
  (`self.HandleFightStyleChangedBP`)
  (add `AP_AttributeSet.OnHealthPercentChanged` _stats (`|CreateDelegate` :!event `HandleHealthPercentChangedBP`))
  (add `AP_AttributeSet.OnManaPercentChanged` _stats (`|CreateDelegate` :!event `HandleManaPercentChangedBP`))
  (add `AP_AttributeSet.OnDeath` _stats (`|CreateDelegate` :!event `HandleDeathBP`))
  (add `AP_AttributeSet.OnLevelUp` _stats (`|CreateDelegate` :!event `HandleLevelUpBP`))
  (add `self.OnRespawn` (`|CreateDelegate` :!event `HandleRespawnBP`))
  (set `self.RespawnLocation` (`self.K2_GetActorLocation`))
  (bind _asfloating_resource_bar (cast `/Game/Common/UI/FloatingResourceBar` (`WidgetComponent.GetUserWidgetObject` (`self.OverheadDisplay`)))
    (:`then`
      (set `self.ResourceBar` _asfloating_resource_bar))
    (:`CastFailed`
      _))
  (`SkinnedMeshComponent.SetLeaderPoseComponent` (`self.Axe_Mesh`) (`self.Mesh`) false)
  (`SkinnedMeshComponent.SetLeaderPoseComponent` (`self.Sword_Mesh`) (`self.Mesh`) false)
  (`SkinnedMeshComponent.SetLeaderPoseComponent` (`self.Bow_Mesh`) (`self.Mesh`) false)
  (`SkinnedMeshComponent.SetLeaderPoseComponent` (`self.Dagger_Mesh`) (`self.Mesh`) false)
  (`SkinnedMeshComponent.SetLeaderPoseComponent` (`self.Dual_Mesh`) (`self.Mesh`) false)
  (`SkinnedMeshComponent.SetLeaderPoseComponent` (`self.Katana_Mesh`) (`self.Mesh`) false)
  (add `self.OnFightStyleChanged` (`|CreateDelegate` :!event `HandleFightStyleChangedBP`))
  (add `TeamAgent.OnCloakStarted` _teamagent (`|CreateDelegate` :!event `HandleOnCloakStartedBP`))
  (add `TeamAgent.OnCloakFinished` _teamagent (`|CreateDelegate` :!event `HandleOnCloakFinishedBP`)))

(fn `HandleDeathBP`
  (`PrimitiveComponent.SetCollisionEnabled` (`self.QueryBox`) "NoCollision")
  (`SceneComponent.SetVisibility` (`self.OverheadDisplay`) false false)
  (`self.K2_SetActorLocation` (+ (`self.RespawnLocation`) (0.0 0.0 99999.0))))

(fn `HandleFightStyleChangedBP`
  (bind _katana_mesh (`self.Katana_Mesh`))
  (bind _returnvalue (select `EFightStyle` (`self.FightStyle`) :`Axe` (`self.Axe_Mesh`) :`Bow` (`self.Bow_Mesh`) :`Dagger` (`self.Dagger_Mesh`) :`DualSword` (`self.Dual_Mesh`) :`Katana1` _katana_mesh :`Katana2` _katana_mesh :`Katana3` _katana_mesh :`MagicStaff` (`self.Wizard_Orb`) :`SwordAndShield` (`self.Sword_Mesh`) :!type "SceneComponent Object Reference"))
  (`SceneComponent.SetVisibility` (`self.Axe_Mesh`) false true)
  (`SceneComponent.SetVisibility` (`self.Sword_Mesh`) false true)
  (`SceneComponent.SetVisibility` (`self.Bow_Mesh`) false true)
  (`SceneComponent.SetVisibility` (`self.Dagger_Mesh`) false true)
  (`SceneComponent.SetVisibility` (`self.Dual_Mesh`) false true)
  (`SceneComponent.SetVisibility` (`self.Katana_Mesh`) false true)
  (`SceneComponent.SetVisibility` (`self.Wizard_Orb`) false true)
  (`SceneComponent.SetVisibility` (`self.TwinSword_L_Mesh`) false true)
  (`SceneComponent.SetVisibility` (`self.TwinSword_R_Mesh`) false true)
  (`/Engine/EditorBlueprintResources/StandardMacros.IsValid` _returnvalue
    (:`Is Valid`
      (`SceneComponent.SetVisibility` _returnvalue true true))
    (:`Is Not Valid`
      _))
  (set `CharacterMovementComponent.bOrientRotationToMovement` (select `EFightStyle` (`self.FightStyle`) :`BareHand` true :`Axe` true :`AxeMelee` true :`DualSword` true :`Katana1` true :`Katana2` true :`Katana3` true :`SwordAndShield` true :`SwordNoShield` true :`SwordMelee` true) (`self.CharacterMovement`))
  (set `self.JumpMaxCount` (select `EFightStyle` (`self.FightStyle`) :`BareHand` 1 :`Axe` 1 :`Bow` 1 :`DualSword` 1 :`Katana1` 1 :`Katana2` 1 :`Katana3` 1 :`MagicStaff` 1 :`SwordAndShield` 1))
  (set `CharacterMovementComponent.bAllowPhysicsRotationDuringAnimRootMotion` (select `EFightStyle` (`self.FightStyle`) :`Axe` true) (`self.CharacterMovement`)))

(fn `HandleHealthPercentChangedBP`
  (params (NewPercent :type "Float (double-precision)"))
  (bind _stats (`self.Stats`))
  (`/Game/Common/UI/FloatingResourceBar.SetHPPercent` (`self.ResourceBar`) NewPercent)
  (`KismetSystemLibrary.PrintString` (`KismetStringLibrary.Concat_StrStr` "health changed " (`KismetStringLibrary.Conv_DoubleToString` (`.CurrentValue` (break `GameplayAttributeData` (`AP_AttributeSet.Health` _stats)))) "/" (`KismetStringLibrary.Conv_DoubleToString` (`.CurrentValue` (break `GameplayAttributeData` (`AP_AttributeSet.MaxHealth` _stats)))))))

(fn `HandleLevelUpBP`)

(fn `HandleManaPercentChangedBP`
  (params (NewPercent :type "Float (double-precision)"))
  (bind _stats (`self.Stats`))
  (`/Game/Common/UI/FloatingResourceBar.SetMPPercent` (`self.ResourceBar`) NewPercent)
  (`KismetSystemLibrary.PrintString` (`KismetStringLibrary.Concat_StrStr` "mana changed " (`KismetStringLibrary.Conv_DoubleToString` (`.CurrentValue` (break `GameplayAttributeData` (`AP_AttributeSet.Mana` _stats)))) "/" (`KismetStringLibrary.Conv_DoubleToString` (`.CurrentValue` (break `GameplayAttributeData` (`AP_AttributeSet.MaxMana` _stats)))))))

(fn `HandleOnCloakFinishedBP`
  (params (Level :type "ECloakingLevel Enum" :default "None"))
  (`self.HandleFightStyleChangedBP`))

(fn `HandleOnCloakStartedBP`
  (params (Level :type "ECloakingLevel Enum" :default "None"))
  (switch `ECloakingLevel` Level
    (:`Vanished`
      (`SceneComponent.SetVisibility` (`self.Mesh`) false true))))

(fn `HandleRespawnBP`
  (`PrimitiveComponent.SetCollisionEnabled` (`self.QueryBox`) "QueryOnly")
  (`SceneComponent.SetVisibility` (`self.OverheadDisplay`) true false)
  (`self.K2_SetActorLocation` (`self.RespawnLocation`)))

(fn `UpdateDash`)

(fn `UserConstructionScript`)
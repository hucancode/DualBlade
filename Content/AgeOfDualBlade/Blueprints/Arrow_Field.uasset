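; Arrow_Field is a timed area actor that rains Arrow_Field_Stem actors around its location until its lifespan expires.
; On BeginPlay it starts a looping delay that spawns each stem at a random X/Y offset within a square range, raised by a set height.
; Each stem gets a randomized lifespan, a falling time derived from it, and the field's parent ability system and damage class.
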(event `self.ReceiveBeginPlay`
  (bind _range (`self.Range`))
  (bind _returnvalue (* _range -1.0))
  (`self.SetLifeSpan` (`self.Lifespan`))
  (`KismetSystemLibrary.Delay` (`self.SpawnInterval`) :!label _label)
  (bind _returnvalue_2 (`|SpawnActorFromClass` "/Game/AgeOfDualBlade/Blueprints/Arrow_Field_Stem.Arrow_Field_Stem_C" (`KismetMathLibrary.MakeTransform` (`KismetMathLibrary.MakeVector` (+ (.x (`self.K2_GetActorLocation`)) (`KismetMathLibrary.RandomFloatInRange` _returnvalue _range)) (+ (.y (`self.K2_GetActorLocation`)) (`KismetMathLibrary.RandomFloatInRange` _returnvalue _range)) (+ (.z (`self.K2_GetActorLocation`)) (`self.Height`)))) "AlwaysSpawn" "OverrideRootScale" null null))
  (bind _output_get (set `/Game/AgeOfDualBlade/Blueprints/Arrow_Field_Stem.Lifespan` (`KismetMathLibrary.RandomFloatInRange` 1.5 1.8) _returnvalue_2))
  (set `/Game/AgeOfDualBlade/Blueprints/Arrow_Field_Stem.FallingTime` (- _output_get 1.2) _returnvalue_2)
  (set `/Game/AgeOfDualBlade/Blueprints/Arrow_Field_Stem.ParentAbilitySystem` (`self.ParentAbilitySystem`) _returnvalue_2)
  (set `/Game/AgeOfDualBlade/Blueprints/Arrow_Field_Stem.DamageClass` (`self.DamageClass`) _returnvalue_2)
  (goto _label))

(fn `UserConstructionScript`)
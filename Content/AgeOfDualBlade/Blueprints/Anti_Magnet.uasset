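; Anti_Magnet is an actor that pushes a list of actors away from its location each tick, then destroys itself once the list is empty.
; DoRepulse moves each listed actor outward at RepulsiveForce scaled by delta time, without sweeping, and drops any beyond AcceptanceRange.
; For dropped actors that are AP_Hero, RemoveEffect removes active gameplay effects matching the granted tags on RepulsedClass defaults.
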(event `self.ReceiveTick`
  (params (DeltaSeconds :type "Float (single-precision)"))
  (if (== (`KismetArrayLibrary.Array_Length` (`self.Actor_To_Repulse`)) 0)
    (`self.K2_DestroyActor`)
    (else
      (`self.DoRepulse` DeltaSeconds))))

(fn `DoRepulse`
  (params (DeltaTime :type "Float (double-precision)"))
  (locals (MagnetLocation :type "Vector Structure") (ActorLocation :type "Vector Structure") (D :type "Vector Structure"))
  (set `local.MagnetLocation` (`self.K2_GetActorLocation`))
  (bind (_arrayindex _arrayelement) (`/Engine/EditorBlueprintResources/StandardMacros.ReverseForEachLoop` (`self.Actor_To_Repulse`))
    (:`LoopBody`
      (set `local.ActorLocation` (`self.K2_GetActorLocation` _arrayelement))
      (set `local.D` (- (`local.ActorLocation`) (`local.MagnetLocation`)))
      (if (> (`KismetMathLibrary.VSize` (`local.D`)) (`self.Acceptance_Range`))
        (`self.RemoveEffect` _arrayelement)
        (`KismetArrayLibrary.Array_Remove` (`self.Actor_To_Repulse`) _arrayindex)
        (else
          (`self.K2_SetActorLocation` _arrayelement (+ (`local.ActorLocation`) (* (* (`KismetMathLibrary.Normal` (`local.D`)) (`self.Repulsive_Force`)) (`local.DeltaTime`))) false false))))))

(fn `RemoveEffect`
  (params (Actor :type "Actor Object Reference"))
  (bind _asap_hero (cast `AP_Hero` Actor))
  (`AbilitySystemComponent.RemoveActiveEffectsWithTags` (`AbilitySystemBlueprintLibrary.GetAbilitySystemComponent` _asap_hero) (`.CombinedTags` (break `InheritedTagContainer` (`.InheritableOwnedTagsContainer` (defaults `/Game/AgeOfDualBlade/Blueprints/Magnet` (`self.Repulsed_Class`)))))))

(fn `UserConstructionScript`)
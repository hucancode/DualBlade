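; Ability object for Iggy's M1 Phoenix, a physics-driven projectile lobbed in a steep arc from its facing direction.
; On init it makes its sphere query-only and launches the mesh with a mass-independent impulse angled 75 degrees off forward.
; Tick applies a strong constant downward acceleration to bend the flight.
; The sphere overlap handler is empty, and an older lerp-based parabolic path with its helper functions is left disconnected.
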(event `self.OnInit`
  (`parent.OnInit`)
  (`PrimitiveComponent.SetCollisionEnabled` (`self.Sphere`) "QueryOnly")
  (`PrimitiveComponent.AddImpulse` (`self.Mesh`) (* (`KismetMathLibrary.RotateAngleAxis` (`self.GetActorForwardVector`) -75.0 (`self.GetActorRightVector`)) (`self.ImpulseStrength`)) "None" true))

(event `CalculatePath`
  (bind _returnvalue (`self.K2_GetActorLocation`))
  (set `self.OriginalLocation` _returnvalue)
  (set `self.GoalLocation` (+ (* (`self.GetActorForwardVector`) (`self.Range`)) _returnvalue)))

(event `self.ReceiveTick`
  (params (DeltaSeconds :type "Float (single-precision)"))
  (`PrimitiveComponent.AddForce` (`self.Mesh`) (0.0 0.0 -6000.0) "None" true))

(event `self.Sphere.OnComponentBeginOverlap`
  (params (OverlappedComponent :type "PrimitiveComponent Object Reference") (OtherActor :type "Actor Object Reference") (OtherComp :type "PrimitiveComponent Object Reference") (OtherBodyIndex :type Integer) (bFromSweep :type Boolean) (SweepResult :type "HitResult Structure (by ref)")))

(fn `UserConstructionScript`)
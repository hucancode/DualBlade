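; Arrow projectile for a bow ability that applies a gameplay effect damage spec to what it hits.
; Tick moves it forward at Speed without sweeping, and it expires after Lifespan.
; On sphere overlap, targets with an ability system component receive DamageHandle through AbilitySystem, then the arrow destroys itself.
; The static-mesh destroy check tests OverlappedComponent, its own sphere, rather than the other component.
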(event `self.ReceiveBeginPlay`
  (`self.SetLifeSpan` (`self.Lifespan`)))

(event `self.ReceiveTick`
  (params (DeltaSeconds :type "Float (single-precision)"))
  (`self.K2_SetActorLocation` (+ (`self.K2_GetActorLocation`) (* (`self.GetActorForwardVector`) (* (`self.Speed`) DeltaSeconds)))))

(event `self.Sphere.OnComponentBeginOverlap`
  (params (OverlappedComponent :type "PrimitiveComponent Object Reference") (OtherActor :type "Actor Object Reference") (OtherComp :type "PrimitiveComponent Object Reference") (OtherBodyIndex :type Integer) (bFromSweep :type Boolean) (SweepResult :type "HitResult Structure (by ref)"))
  (bind _returnvalue (`AbilitySystemBlueprintLibrary.GetAbilitySystemComponent` OtherActor))
  (`/Engine/EditorBlueprintResources/StandardMacros.IsValid` _returnvalue
    (:`Is Valid`
      (`AbilitySystemComponent.BP_ApplyGameplayEffectSpecToTarget` (`self.AbilitySystem`) (`self.DamageHandle`) _returnvalue)
      (`self.K2_DestroyActor` :!label _label))
    (:`Is Not Valid`
      (if (`KismetMathLibrary.ClassIsChildOf` (`GameplayStatics.GetObjectClass` OverlappedComponent) "/Script/Engine.StaticMeshComponent")
        (goto _label)))))

(fn `UserConstructionScript`)
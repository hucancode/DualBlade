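; Shield_Projectile is an ability object that flies in a straight line while spinning and damages fight units it overlaps.
; On BeginPlay it sets its lifespan and caches its forward vector, then Tick moves it along that direction without sweeping and spins its yaw.
; Box overlaps with AP_FightUnit actors apply the DamageHandle gameplay effect spec through ParentAbilitySystem, without destroying the projectile.
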(event `self.ReceiveBeginPlay`
  (`self.SetLifeSpan` (`self.Lifespan`))
  (set `self.ForwardVector` (`self.GetActorForwardVector`)))

(event `self.ReceiveTick`
  (params (DeltaSeconds :type "Float (single-precision)"))
  (`self.K2_SetActorLocation` (+ (`self.K2_GetActorLocation`) (* (`self.ForwardVector`) (* (`self.Speed`) DeltaSeconds))))
  (`self.K2_SetActorRotation` (`KismetMathLibrary.MakeRotator` 0.0 0.0 (+ (.yaw (`self.K2_GetActorRotation`)) (* DeltaSeconds (`self.SpinSpeed`))))))

(event `self.Box.OnComponentBeginOverlap`
  (params (OverlappedComponent :type "PrimitiveComponent Object Reference") (OtherActor :type "Actor Object Reference") (OtherComp :type "PrimitiveComponent Object Reference") (OtherBodyIndex :type Integer) (bFromSweep :type Boolean) (SweepResult :type "HitResult Structure (by ref)"))
  (bind _parentabilitysystem (`self.ParentAbilitySystem`))
  (bind _asap_fight_unit (cast `AP_FightUnit` OtherActor))
  (`/Engine/EditorBlueprintResources/StandardMacros.IsValid` _parentabilitysystem
    (:`Is Valid`
      (`AbilitySystemComponent.BP_ApplyGameplayEffectSpecToTarget` _parentabilitysystem (`self.DamageHandle`) (`AbilitySystemBlueprintLibrary.GetAbilitySystemComponent` _asap_fight_unit)))))

(fn `UserConstructionScript`)
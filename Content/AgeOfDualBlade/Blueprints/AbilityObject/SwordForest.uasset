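; SwordForest is an ability object actor that animates its static meshes popping into view, then removes itself after a short fixed lifespan.
; Each Tick rescales every StaticMeshComponent, with double height on Z, using time since creation.
; The scale grows linearly from zero to PopInSize over PopInTime, then eases linearly to the base size over RecoverTime and holds there.
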(event `self.ReceiveBeginPlay`
  (`self.SetLifeSpan` 4.0))

(event `self.ReceiveTick`
  (params (DeltaSeconds :type "Float (single-precision)"))
  (bind _returnvalue (`self.GetGameTimeSinceCreation`))
  (for _array_element (`self.K2_GetComponentsByClass` "/Script/Engine.StaticMeshComponent")
    (`SceneComponent.SetRelativeScale3D` _array_element (* (1.0 1.0 2.0) (`KismetMathLibrary.SelectFloat` (`KismetMathLibrary.Lerp` 0.0 (`self.PopInSize`) (/ _returnvalue (`self.PopInTime`))) (`KismetMathLibrary.Lerp` (`self.PopInSize`) 1.0 (`KismetMathLibrary.FClamp` (/ (- (`self.GetGameTimeSinceCreation`) (`self.PopInTime`)) (`self.RecoverTime`)))) (< _returnvalue (`self.PopInTime`)))))))

(fn `UserConstructionScript`)
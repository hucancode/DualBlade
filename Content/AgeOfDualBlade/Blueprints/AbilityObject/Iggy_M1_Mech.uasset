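; Iggy_M1_Mech is an ability object that registers hits through a sphere overlap and visually breaks down shortly before its lifespan ends.
; On init it enables query-only sphere collision, passes overlaps to OnHit, and schedules Collapse half a second before expiry.
; Collapse disables collision and particles, after which Tick skips parent logic and randomly rescales the mesh each frame as a flicker effect.
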(event `self.ReceiveTick`
  (params (DeltaSeconds :type "Float (single-precision)"))
  (if (`self.IsCollapsing`)
    (`SceneComponent.SetRelativeScale3D` (`self.Mesh`) (`KismetMathLibrary.Conv_DoubleToVector` (`KismetMathLibrary.RandomFloat`)))
    (else
      (`parent.ReceiveTick` DeltaSeconds))))

(event `self.OnInit`
  (`parent.OnInit`)
  (`PrimitiveComponent.SetCollisionEnabled` (`self.Sphere_0`) "QueryOnly")
  (`KismetSystemLibrary.Delay` (- (`self.GetLifeSpan`) 0.5))
  (`self.Collapse`))

(event `self.Sphere_0.OnComponentBeginOverlap`
  (params (OverlappedComponent :type "PrimitiveComponent Object Reference") (OtherActor :type "Actor Object Reference") (OtherComp :type "PrimitiveComponent Object Reference") (OtherBodyIndex :type Integer) (bFromSweep :type Boolean) (SweepResult :type "HitResult Structure (by ref)"))
  (`self.OnHit` OtherActor OtherComp))

(fn `Collapse`
  (`PrimitiveComponent.SetCollisionEnabled` (`self.Sphere_0`) "NoCollision")
  (set `self.IsCollapsing` true)
  (`ActorComponent.Deactivate` (`self.ParticleSystem`)))

(fn `UserConstructionScript`)
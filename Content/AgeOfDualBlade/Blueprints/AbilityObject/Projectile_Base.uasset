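; Base projectile for ability objects that flies straight ahead and deals damage through the Gameplay Ability System.
; Each tick it moves along its forward vector at Speed by setting its location without sweep.
; On hit it ignores actors sharing its own ability system, applies the DamageHandle effect spec to any other ability system, then destroys itself.
; Static mesh components without an ability system also destroy it, and OnInit is empty.
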(event `OnInit`)

(event `self.ReceiveTick`
  (params (DeltaSeconds :type "Float (single-precision)"))
  (`self.K2_SetActorLocation` (+ (`self.K2_GetActorLocation`) (* (`self.GetActorForwardVector`) (* (`self.Speed`) DeltaSeconds)))))

(event `OnHit`
  (params (OtherActor :type "Actor Object Reference") (OtherComponent :type "PrimitiveComponent Object Reference"))
  (bind _returnvalue (`AbilitySystemBlueprintLibrary.GetAbilitySystemComponent` OtherActor))
  (if (not (== _returnvalue (`self.AbilitySystem`)))
    (`/Engine/EditorBlueprintResources/StandardMacros.IsValid` _returnvalue
      (:`Is Valid`
        (`self.DealDamageTo` _returnvalue)
        (`self.K2_DestroyActor` :!label _label))
      (:`Is Not Valid`
        (if (`KismetMathLibrary.ClassIsChildOf` (`GameplayStatics.GetObjectClass` OtherComponent) "/Script/Engine.StaticMeshComponent")
          (goto _label))))))

(event `DealDamageTo`
  (params (Target :type "AbilitySystemComponent Object Reference"))
  (`AbilitySystemComponent.BP_ApplyGameplayEffectSpecToTarget` (`self.AbilitySystem`) (`self.DamageHandle`) Target))

(fn `UserConstructionScript`)
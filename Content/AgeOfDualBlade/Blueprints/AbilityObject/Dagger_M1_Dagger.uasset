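; Dagger_M1_Dagger is an ability object Blueprint, apparently the dagger spawned by a Dagger M1 attack.
; Each tick, after the parent's tick, it interpolates the mesh scale from InitialScale toward FinalScale as its remaining lifespan runs out, holding FinalScale when the initial lifespan is negligible.
; Box overlaps are forwarded to OnHit with the other actor and component.
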(event `self.ReceiveTick`
  (params (DeltaSeconds :type "Float (single-precision)"))
  (bind _initiallifespan (`self.InitialLifeSpan`))
  (`parent.ReceiveTick` DeltaSeconds)
  (`SceneComponent.SetRelativeScale3D` (`self.Mesh`) (`KismetMathLibrary.VLerp` (`self.FinalScale`) (`self.InitialScale`) (select `bool` (<= _initiallifespan 0.1) :`false` (/ (`self.GetLifeSpan`) _initiallifespan) :`true` 0.0))))

(event `self.Box.OnComponentBeginOverlap`
  (params (OverlappedComponent :type "PrimitiveComponent Object Reference") (OtherActor :type "Actor Object Reference") (OtherComp :type "PrimitiveComponent Object Reference") (OtherBodyIndex :type Integer) (bFromSweep :type Boolean) (SweepResult :type "HitResult Structure (by ref)"))
  (`self.OnHit` OtherActor OtherComp))

(fn `UserConstructionScript`)
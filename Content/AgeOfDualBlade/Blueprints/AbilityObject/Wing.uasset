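; Wing actor for an ability object that animates six TwinSword components and a TwinSword component as a flapping wing.
; Tick advances a time value by AnimationSpeed and folds it into a triangle-wave Spread between 0 and 30.
; UpdateAnimation, also run by the construction script, applies the X/Z offsets and Spread pitch to the six swords.
; It also scales TwinSword with a clamped minimum and pitches it further as Spread grows.
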(event `self.ReceiveTick`
  (params (DeltaSeconds :type "Float (single-precision)"))
  (bind _output_get (set `self.Time` (+ (`self.Time`) (* DeltaSeconds (`self.AnimationSpeed`)))))
  (set `self.Spread` (`KismetMathLibrary.Abs` (- (mod _output_get 60.0) 30.0)))
  (`self.UpdateAnimation`))

(fn `UpdateAnimation`
  (bind _twinsword1 (`self.TwinSword1`))
  (bind _returnvalue (/ (`self.Spread`) 30.0))
  (`SceneComponent.K2_SetRelativeLocation` _twinsword1 (`KismetMathLibrary.MakeVector` (`self.X_Offset`) 0.0 (`self.Z_Offset`)) false false)
  (`SceneComponent.K2_SetRelativeLocation` (`self.TwinSword2`) (`KismetMathLibrary.MakeVector` (`self.X_Offset`) 0.0 (`self.Z_Offset`)) false false)
  (`SceneComponent.K2_SetRelativeLocation` (`self.TwinSword3`) (`KismetMathLibrary.MakeVector` (`self.X_Offset`) 0.0 (`self.Z_Offset`)) false false)
  (`SceneComponent.K2_SetRelativeLocation` (`self.TwinSword4`) (`KismetMathLibrary.MakeVector` (`self.X_Offset`) 0.0 (`self.Z_Offset`)) false false)
  (`SceneComponent.K2_SetRelativeLocation` (`self.TwinSword5`) (`KismetMathLibrary.MakeVector` (`self.X_Offset`) 0.0 (`self.Z_Offset`)) false false)
  (`SceneComponent.K2_SetRelativeLocation` (`self.TwinSword6`) (`KismetMathLibrary.MakeVector` (`self.X_Offset`) 0.0 (`self.Z_Offset`)) false false)
  (`SceneComponent.K2_SetRelativeRotation` _twinsword1 (`KismetMathLibrary.MakeRotator` 0.0 (`self.Spread`)) false false)
  (`SceneComponent.K2_SetRelativeRotation` (`self.TwinSword4`) (`KismetMathLibrary.MakeRotator` 0.0 (`self.Spread`)) false false)
  (`SceneComponent.K2_SetRelativeRotation` (`self.TwinSword3`) (`KismetMathLibrary.MakeRotator` 0.0 (`self.Spread`)) false false)
  (`SceneComponent.K2_SetRelativeRotation` (`self.TwinSword2`) (`KismetMathLibrary.MakeRotator` 0.0 (`self.Spread`)) false false)
  (`SceneComponent.K2_SetRelativeRotation` (`self.TwinSword6`) (`KismetMathLibrary.MakeRotator` 0.0 (`self.Spread`)) false false)
  (`SceneComponent.K2_SetRelativeRotation` (`self.TwinSword5`) (`KismetMathLibrary.MakeRotator` 0.0 (`self.Spread`)) false false)
  (`SceneComponent.SetRelativeScale3D` (`self.TwinSword`) (`KismetMathLibrary.Conv_DoubleToVector` (`KismetMathLibrary.FClamp` _returnvalue 0.3 1.0)))
  (`SceneComponent.K2_SetRelativeRotation` (`self.TwinSword`) (`KismetMathLibrary.MakeRotator` 0.0 (- (* _returnvalue -45.0) 45.0)) false false))

(fn `UserConstructionScript`
  (`self.UpdateAnimation`))
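; Axe ability object that exists in the world for a limited lifespan and is tied to a buff on its parent ability system.
; Tick moves the Axe component from an original to a destination relative location, interpolating on time since creation over a falling time without sweep.
; When the actor is destroyed, it removes active effects matching the buff class's granted tags from the parent ability system.
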(event `self.ReceiveBeginPlay`
  (`self.SetLifeSpan` (`self.Lifespan`)))

(event `self.ReceiveTick`
  (params (DeltaSeconds :type "Float (single-precision)"))
  (`SceneComponent.K2_SetRelativeLocation` (`self.Axe`) (`KismetMathLibrary.VLerp` (`self.Original`) (`self.Destination`) (`KismetMathLibrary.FMin` (/ (`self.GetGameTimeSinceCreation`) (`self.Falling_Time`)) 1.0)) false false))

(event `self.ReceiveDestroyed`
  (`self.RemoveBuff`))

(fn `RemoveBuff`
  ;[1 1 1] then setup fight style again
  (`AbilitySystemComponent.RemoveActiveEffectsWithGrantedTags` (`self.ParentAbilitySystem`) (`.CombinedTags` (break `InheritedTagContainer` (`.InheritableOwnedTagsContainer` (defaults `/Game/AgeOfDualBlade/Blueprints/AbilityObject/Axe_In_World` (`self.Buff_Class`)))))))

(fn `UserConstructionScript`)
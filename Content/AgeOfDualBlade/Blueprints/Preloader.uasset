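; Preloader actor that asynchronously loads a soft-referenced animation montage and particle asset when play begins.
; The particle load starts from the montage load's immediate output, so both requests run concurrently.
; Each completion stores the loaded asset in a variable and prints its name, with both messages labelled as montage preloads.
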(event `self.ReceiveBeginPlay`
  (bind _object (`|LoadAsset` (`self.AnimMontage`))
    (:`then`
      (bind _object_2 (`|LoadAsset` (`self.Particle`))
        (:`Completed`
          (set `self.NewVar_1` _object_2)
          (`KismetSystemLibrary.PrintString` (`KismetStringLibrary.Concat_StrStr` "preload montage finished" (`KismetSystemLibrary.GetDisplayName` _object_2))))))
    (:`Completed`
      (set `self.NewVar_0` _object)
      (`KismetSystemLibrary.PrintString` (`KismetStringLibrary.Concat_StrStr` "preload montage finished" (`KismetSystemLibrary.GetObjectName` _object))))))

(fn `UserConstructionScript`)
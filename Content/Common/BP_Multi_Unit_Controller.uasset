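; RTS player controller that pans the camera pawn, selects team units through the RTS HUD, and issues move, stop, hold and ability orders.
; Abilities enter a crosshair targeting mode for unit- or ground-target skills, while others fire immediately on the leader, the first selected hero.
; Orders are written to each unit's AI Blackboard as target, skill slot, cast range and state; basic attacks go to all selected units, other targeted skills only to the leader.
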(event `InputAxis|CameraX`
  (params (AxisValue :type "Float (single-precision)"))
  (bind _returnvalue (`self.K2_GetPawn`))
  (`Pawn.AddMovementInput` _returnvalue (`SceneComponent.GetRightVector` (`Actor.RootComponent` _returnvalue)) AxisValue false))

(event `self.ReceiveBeginPlay`)

(event `InputAxis|CameraY`
  (params (AxisValue :type "Float (single-precision)"))
  (bind _returnvalue (`self.K2_GetPawn`))
  (`Pawn.AddMovementInput` _returnvalue (`SceneComponent.GetForwardVector` (`Actor.RootComponent` _returnvalue)) AxisValue false))

(event `InputAction|CancelTargeting`
  (params (Key :type "Key Structure"))
  (:`Pressed`
    (if (`self.Targeting`)
      (`self.CancelTargeting`)
      (else
        (`self.Move`)))))

(event `InputAction|ConfirmTargeting`
  (params (Key :type "Key Structure"))
  (bind _targeting (`self.Targeting`))
  (:`Pressed`
    (if (not _targeting)
      (bind _asrts_hud (cast `/Game/Common/UI/RTS_HUD` (`self.GetHUD`)))
      (`/Game/Common/UI/RTS_HUD.MouseClicked` _asrts_hud null Key)))
  (:`Released`
    (if _targeting
      (`self.ConfirmTargeting`)
      (else
        (bind _asrts_hud_2 (cast `/Game/Common/UI/RTS_HUD` (`self.GetHUD`)))
        (`/Game/Common/UI/RTS_HUD.MouseReleased` _asrts_hud_2 null Key)))))

(event `InputAction|WeaponAbility`
  (params (Key :type "Key Structure"))
  (:`Pressed`
    (`self.ActivateAbility` 0)))

(event `InputAction|UseAbility1`
  (params (Key :type "Key Structure"))
  (:`Pressed`
    (`self.ActivateAbility` 1)))

(event `InputAction|UseAbility2`
  (params (Key :type "Key Structure"))
  (:`Pressed`
    (`self.ActivateAbility` 2)))

(event `InputAction|UseAbility3`
  (params (Key :type "Key Structure"))
  (:`Pressed`
    (`self.ActivateAbility` 3)))

(event `InputAction|UseAbility4`
  (params (Key :type "Key Structure"))
  (:`Pressed`
    (`self.ActivateAbility` 4)))

(event `InputAction|UseAbility5`
  (params (Key :type "Key Structure"))
  (:`Pressed`
    (`self.ActivateAbility` 5)))

(event `InputAction|UseAbility6`
  (params (Key :type "Key Structure"))
  (:`Pressed`
    (`self.ActivateAbility` 6)))

(event `InputAction|Hold`
  (params (Key :type "Key Structure"))
  (:`Pressed`
    (`self.Hold`)))

(event `InputAction|Stop`
  (params (Key :type "Key Structure"))
  (:`Pressed`
    (`self.Stop`)))

(event `ActivateAbility`
  (params (AbilitySlot :type Integer))
  (set `self.TargetingAbility` AbilitySlot)
  (`self.EnterTargeting`))

(fn `CancelTargeting`
  (set `self.Targeting` false)
  (set `self.CurrentMouseCursor` "Default"))

(fn `ClearTargetInfo`
  (params (Unit :type "Actor Object Reference"))
  (bind _returnvalue (`AIBlueprintHelperLibrary.GetBlackboard` Unit))
  (`BlackboardComponent.SetValueAsInt` _returnvalue (`self.SkillToCast_KeyName`) -1)
  (`BlackboardComponent.ClearValue` _returnvalue (`self.TargetActor_KeyName`))
  (`BlackboardComponent.SetValueAsFloat` _returnvalue (`self.CastRange_KeyName`) 99999.0)
  (`BlackboardComponent.ClearValue` _returnvalue (`self.TargetLocation_KeyName`)))

(fn `ConfirmTargeting`
  (locals (IsUnitTarget :type Boolean) (IsGroundTarget :type Boolean) (IsBasicAttack :type Boolean))
  (bind _returnvalue (`GameplayStatics.GetObjectClass` (`AP_Hero.GetAbility` (`self.LeaderUnit`) (`self.TargetingAbility`))))
  (bind _output_get (set `local.IsBasicAttack` (== (`self.TargetingAbility`) 0)))
  (if _output_get
    (bind (_hit _actor) (`self.MouseHitTestUnit`))
    (if _hit
      (for _array_element (`self.ControlledUnits`)
        (`self.ClearTargetInfo` _array_element)
        (`self.WriteActorTarget` _actor _array_element)
        (`self.WriteSkillToCast` (`self.TargetingAbility`) _array_element)
        (`self.WriteState` "NewEnumerator7" _array_element)
        (`self.StopAllMontage` _array_element))
      (set `self.Targeting` false)
      (set `self.CurrentMouseCursor` "Default")
      (else
        (bind (_hit_2 _location) (`self.MouseHitTestFloor`))
        (if _hit_2
          (for _array_element_2 (`self.ControlledUnits`)
            (`self.ClearTargetInfo` _array_element_2)
            (`self.WriteLocationTarget` _location _array_element_2)
            (`self.WriteSkillToCast` (`self.TargetingAbility`) _array_element_2)
            (`self.WriteState` "NewEnumerator6" _array_element_2)
            (`self.StopAllMontage` _array_element_2))
          (set `self.Targeting` false)
          (set `self.CurrentMouseCursor` "Default"))))
    (elif (`KismetMathLibrary.ClassIsChildOf` _returnvalue "/Game/AgeOfDualBlade/Abilities/Core/Base/Unit_Target_Skill.Unit_Target_Skill_C")
      (bind (_hit_3 _actor_2) (`self.MouseHitTestUnit`))
      (if _hit_3
        (`self.ClearTargetInfo` (`self.LeaderUnit`))
        (`self.WriteActorTarget` _actor_2 (`self.LeaderUnit`))
        (`self.WriteSkillToCast` (`self.TargetingAbility`) (`self.LeaderUnit`) :!label _label)
        (`self.WriteState` "NewEnumerator3" (`self.LeaderUnit`))
        (`Character.StopAnimMontage` (`self.LeaderUnit`) null)
        (set `self.Targeting` false)
        (set `self.CurrentMouseCursor` "Default"))
      (elif (`KismetMathLibrary.ClassIsChildOf` _returnvalue "/Game/AgeOfDualBlade/Abilities/Core/Base/Ground_Target_Skill.Ground_Target_Skill_C")
        (bind (_hit_4 _location_2) (`self.MouseHitTestFloor`))
        (if _hit_4
          (`self.ClearTargetInfo` (`self.LeaderUnit`))
          (`self.WriteLocationTarget` _location_2)
          (goto _label))))))

(fn `EnterTargeting`
  (locals (IsGroundTarget :type Boolean) (IsUnitTarget :type Boolean))
  (if (`AP_Hero.CanActivateAbility` (`self.LeaderUnit`) (`self.TargetingAbility`))
    (bind _result (`self.GetAbilityInfo`))
    (bind _returnvalue (`GameplayStatics.GetObjectClass` _result))
    (set `local.IsUnitTarget` (`KismetMathLibrary.ClassIsChildOf` _returnvalue "/Game/AgeOfDualBlade/Abilities/Core/Base/Unit_Target_Skill.Unit_Target_Skill_C"))
    (set `local.IsGroundTarget` (`KismetMathLibrary.ClassIsChildOf` _returnvalue "/Game/AgeOfDualBlade/Abilities/Core/Base/Ground_Target_Skill.Ground_Target_Skill_C"))
    (if (or (`local.IsUnitTarget`) (`local.IsGroundTarget`))
      (`KismetSystemLibrary.PrintString` "enter targeting")
      (set `self.CurrentMouseCursor` "Crosshairs")
      (set `self.Targeting` true)
      (else
        (`KismetSystemLibrary.PrintString` (`KismetStringLibrary.Concat_StrStr` "this skill is, " (`KismetSystemLibrary.GetClassDisplayName` (`GameplayStatics.GetObjectClass` _result)) ", not unit target, not ground target, so skip targeting phase" (`KismetStringLibrary.Conv_IntToString` (`self.TargetingAbility`))))
        (`KismetSystemLibrary.PrintString` "activate skill directly")
        (`AP_Hero.ActivateAbility` (`self.LeaderUnit`) (`self.TargetingAbility`))))))

(fn `GetAbilityInfo`
  (returns (Result :type "GameplayAbility Object Reference"))
  (bind _returnvalue (`AP_Hero.GetAbility` (`self.LeaderUnit`) (`self.TargetingAbility`)))
  (`/Engine/EditorBlueprintResources/StandardMacros.IsValid` _returnvalue
    (:`Is Valid`
      (return _returnvalue))
    (:`Is Not Valid`
      (return null))))

(fn `Hold`
  (for _array_element (`self.ControlledUnits`)
    (`self.ClearTargetInfo` _array_element)
    (`BlackboardComponent.SetValueAsEnum` (`AIBlueprintHelperLibrary.GetBlackboard` _array_element) (`self.AIState_KeyName`) (enumliteral `/Game/Common/AI/AI_BasicState` "NewEnumerator1"))))

(fn `MarkAllUnitSelected`
  (params (Selected :type Boolean))
  (for _array_element (`self.ControlledUnits`)
    (bind _asap_hero (cast `AP_Hero` _array_element))
    (`AP_Hero.SelectHero` _asap_hero Selected)))

(fn `MouseHitTestFloor`
  (returns (Hit :type Boolean) (Location :type "Vector Structure"))
  (bind (_hitresult _returnvalue) (`self.GetHitResultUnderCursorByChannel` "TraceTypeQuery3" false))
  (return _returnvalue (`.Location` (`GameplayStatics.BreakHitResult` _hitresult))))

(fn `MouseHitTestUnit`
  (returns (Hit :type Boolean) (Actor :type "Actor Object Reference"))
  (bind (_hitresult _returnvalue) (`self.GetHitResultUnderCursorByChannel` "TraceTypeQuery11" false))
  (return _returnvalue (`.HitActor` (`GameplayStatics.BreakHitResult` _hitresult))))

(fn `Move`
  (for _array_element (`self.ControlledUnits`)
    (bind _ascharacter (cast `Character` _array_element))
    (`self.StopAllMontage` _ascharacter)
    (`self.ClearTargetInfo` _array_element)
    (bind (_hit _location) (`self.MouseHitTestFloor`))
    (if _hit
      (`GameplayStatics.SpawnEmitterAtLocation` "/Game/LinhiBlade/MouseClickParticle/P_MouseClick.P_MouseClick" _location (struct :`Roll` 90.0) (1.0 1.0 1.0) true "AutoRelease")
      (`self.WriteActorTarget` null _array_element)
      (`self.WriteLocationTarget` _location _array_element)
      (`self.WriteState` "NewEnumerator5" _array_element))))

(fn `SelectUnits`
  (params (Units :type "Array of Actor Object Reference"))
  (`self.MarkAllUnitSelected` false)
  (set `self.ControlledUnits` Units)
  (bind (_arrayindex _arrayelement) (`/Engine/EditorBlueprintResources/StandardMacros.ReverseForEachLoop` (`self.ControlledUnits`))
    (:`LoopBody`
      (bind _returnvalue (message `GameplayTagAssetInterface.HasMatchingGameplayTag` _arrayelement (`self.TeamTag`)))
      (if (not _returnvalue)
        (`KismetArrayLibrary.Array_Remove` (`self.ControlledUnits`) _arrayindex)))
    (:`Completed`
      (`self.MarkAllUnitSelected` true)
      (set `self.LeaderUnit` null)
      (for _array_element (`self.ControlledUnits`)
        (bind _asap_hero (cast `AP_Hero` _array_element))
        (bind _output_get (set `self.LeaderUnit` _asap_hero))
        (`self.OnControlledUnitChanged` _output_get)
        (break)))))

(fn `Stop`
  (for _array_element (`self.ControlledUnits`)
    (bind _ascharacter (cast `Character` _array_element))
    (`Character.StopAnimMontage` _ascharacter null)
    (`self.ClearTargetInfo` null)
    (`BlackboardComponent.SetValueAsEnum` (`AIBlueprintHelperLibrary.GetBlackboard` _array_element) (`self.AIState_KeyName`) (enumliteral `/Game/Common/AI/AI_BasicState` "NewEnumerator1"))))

(fn `StopAllMontage`
  (params (Unit :type "Actor Object Reference"))
  (bind _ascharacter (cast `Character` Unit))
  (`Character.StopAnimMontage` _ascharacter null))

(fn `UserConstructionScript`)

(fn `WriteActorTarget`
  (params (TargetActor :type "Actor Object Reference") (Unit :type "Actor Object Reference"))
  (bind _returnvalue (`AIBlueprintHelperLibrary.GetBlackboard` Unit))
  (bind _targetactor_keyname (`self.TargetActor_KeyName`))
  (`/Engine/EditorBlueprintResources/StandardMacros.IsValid` TargetActor
    (:`Is Valid`
      (`BlackboardComponent.SetValueAsObject` _returnvalue _targetactor_keyname TargetActor))
    (:`Is Not Valid`
      (`BlackboardComponent.ClearValue` _returnvalue _targetactor_keyname))))

(fn `WriteCastRange`
  (params (Range :type "Float (double-precision)") (Unit :type "Actor Object Reference"))
  (`KismetSystemLibrary.PrintString` (`KismetStringLibrary.Concat_StrStr` "write cast range from Controller" (`KismetStringLibrary.Conv_DoubleToString` Range)))
  (`BlackboardComponent.SetValueAsFloat` (`AIBlueprintHelperLibrary.GetBlackboard` Unit) (`self.CastRange_KeyName`) Range))

(fn `WriteLocationTarget`
  (params (TargetLocation :type "Vector Structure") (Unit :type "Actor Object Reference"))
  (`BlackboardComponent.SetValueAsVector` (`AIBlueprintHelperLibrary.GetBlackboard` Unit) (`self.TargetLocation_KeyName`) TargetLocation))

(fn `WriteSkillToCast`
  (params (Slot :type Integer) (Unit :type "Actor Object Reference"))
  (bind _asap_hero (cast `AP_Hero` Unit))
  (`BlackboardComponent.SetValueAsInt` (`AIBlueprintHelperLibrary.GetBlackboard` Unit) (`self.SkillToCast_KeyName`) Slot)
  (bind _returnvalue (`AP_Hero.GetAbility` _asap_hero (`self.TargetingAbility`)))
  (bind _asground_target_skill (cast `/Game/AgeOfDualBlade/Abilities/Core/Base/Ground_Target_Skill` _returnvalue)
    (:`then`
      (bind _result (`/Game/AgeOfDualBlade/Abilities/Core/Base/Ground_Target_Skill.GetCastRange` _asground_target_skill))
      (`self.WriteCastRange` _result Unit))
    (:`CastFailed`
      (bind _asunit_target_skill (cast `/Game/AgeOfDualBlade/Abilities/Core/Base/Unit_Target_Skill` _returnvalue))
      (bind _result_2 (`/Game/AgeOfDualBlade/Abilities/Core/Base/Unit_Target_Skill.GetCastRange` _asunit_target_skill))
      (`self.WriteCastRange` _result_2 Unit))))

(fn `WriteState`
  (params (State :type "/Game/Common/AI/AI_BasicState Enum" :default "NewEnumerator0") (Unit :type "Actor Object Reference"))
  (`BlackboardComponent.SetValueAsEnum` (`AIBlueprintHelperLibrary.GetBlackboard` Unit) (`self.AIState_KeyName`) State))
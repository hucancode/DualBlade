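; BP_Fight_NPC_Controller is the AI controller that drives combat NPCs through the Fight_NPC_Behavior behavior tree.
; On BeginPlay it starts the tree and stores the controlled pawn's location in the blackboard as the camping location.
; Each AI perception target update sets the blackboard enemy to a randomly chosen perceived actor, regardless of which actor triggered the update.
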(event `self.ReceiveBeginPlay`
  (`self.RunBehaviorTree` "/Game/Common/GameMode/AI/Fight_NPC_Behavior.Fight_NPC_Behavior")
  (`BlackboardComponent.SetValueAsVector` (`self.Blackboard`) (`self.CampingLocationKeyName`) (`self.K2_GetActorLocation` (`self.K2_GetPawn`))))

(event `self.AIPerception.OnTargetPerceptionUpdated`
  (params (Actor :type "Actor Object Reference") (Stimulus :type "AIStimulus Structure"))
  (bind _outactors (`AIPerceptionComponent.GetPerceivedActors` (`self.AIPerception`) null))
  (`BlackboardComponent.SetValueAsObject` (`self.Blackboard`) (`self.EnemyKeyName`) (`|GetArrayItem` _outactors (- (`KismetMathLibrary.RandomIntegerInRange` 1 (`KismetArrayLibrary.Array_Length` _outactors)) 1))))

(fn `UserConstructionScript`)
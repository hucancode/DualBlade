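; Player controller for a fight unit: drives movement, jump, facing toward the mouse while moving, and mouse- or key-triggered abilities on the possessed AP_FightUnit.
; Targeted abilities enter a crosshair mode, confirm by deprojected cursor traces for ground or units, and cancel on right click.
; Confirmed targets pass through Server events to the unit as gameplay events with target data; untargeted abilities activate directly.
; It also forwards ability level-ups and shop buy, equip and unequip requests.
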(event `self.ReceivePossess`
  (params (PossessedPawn :type "Pawn Object Reference"))
  (`/Engine/EditorBlueprintResources/ActorMacros.Switch Has Authority`
    (:`Authority`
      (`self.RetrieveControlledPawn`))))

(event `self.ReceiveBeginPlay`)

(event `InputAction|M1`
  (params (Key :type "Key Structure"))
  (:`Pressed`
    (`self.IfPawnValid`
      (:`Is Valid`
        (`self.IsTargeting`
          (:`True`
            (`self.ConfirmWithMouse` (`self.TargetAbility`)))
          (:`False`
            (`self.ConfirmWithMouse` 0)))))))

(event `InputAction|M2`
  (params (Key :type "Key Structure"))
  (:`Pressed`
    (`self.IfPawnValid`
      (:`Is Valid`
        (`self.IsTargeting`
          (:`True`
            (`self.CancelTargeting`))
          (:`False`
            (`self.ConfirmWithMouse` 1)))))))

(event `InputAction|Dash`
  (params (Key :type "Key Structure"))
  (:`Pressed`
    (`self.IfPawnValid`
      (:`Is Valid`
        (`self.ActivateAbility` 3)))))

(event `InputAction|Ultimate`
  (params (Key :type "Key Structure"))
  (:`Pressed`
    (`self.IfPawnValid`
      (:`Is Valid`
        (`self.ActivateAbility` 2)))))

(event `InputAction|Transform`
  (params (Key :type "Key Structure"))
  (:`Pressed`
    (`self.IfPawnValid`
      (:`Is Valid`
        (`self.ActivateAbility` 4)))))

(event `InputAxis|MoveX`
  (params (AxisValue :type "Float (single-precision)"))
  (`self.IfPawnValid`
    (:`Is Valid`
      (`Pawn.AddMovementInput` (`self.K2_GetPawn`) (`KismetMathLibrary.Vector_Forward`) AxisValue false))))

(event `InputAxis|MoveY`
  (params (AxisValue :type "Float (single-precision)"))
  (`self.IfPawnValid`
    (:`Is Valid`
      (`Pawn.AddMovementInput` (`self.K2_GetPawn`) (`KismetMathLibrary.Vector_Right`) AxisValue false))))

(event `InputAction|Jump`
  (params (Key :type "Key Structure"))
  (bind _leaderunit (`self.LeaderUnit`))
  (:`Pressed`
    (`self.IfPawnValid`
      (:`Is Valid`
        (`self.StopMontage` null
          (:`exec`
            (`Character.Jump` _leaderunit))))))
  (:`Released`
    (`self.IfPawnValid`
      (:`Is Valid`
        (`Character.StopJumping` _leaderunit)))))

(event `ActivateAbility`
  (params (AbilitySlot :type Integer))
  (if (`AbilityUser.CanActivateAbility` (`AP_FightUnit.AbilityUser` (`self.LeaderUnit`)) AbilitySlot)
    (`self.EnterTargeting` AbilitySlot)
    (else
      (`KismetSystemLibrary.PrintString` "can't use this ability now"))))

(event `self.ReceiveTick`
  (params (DeltaSeconds :type "Float (single-precision)"))
  (`self.IfPawnValid`
    (:`Is Valid`
      (if (`self.IsMoving`)
        (`self.PlayerFaceToMouse`)))))

(event `ServerSendTargetToAbility`
  (params (Actor :type "Actor Object Reference") (Location :type "Vector Structure") (Ability :type "AP_AbilityBase Object Reference") (AbilityOwner :type "Actor Object Reference"))
  (`self.Send Target to Ability` Actor Location Ability AbilityOwner))

(event `ServerSendTraceGroundToAbility`
  (params (AbilityOwner :type "AP_FightUnit Object Reference") (AbilitySlot :type Integer) (Start :type "Vector Structure") (Direction :type "Vector Structure"))
  (`self.SendLineTraceGroundToAbility` AbilityOwner AbilitySlot Start Direction))

(event `ServerActivateAbilityNoTarget`
  (params (AbilitySlot :type Integer) (AbilityOwner :type "AP_FightUnit Object Reference"))
  ;[1 1 1] doesn't need to run on server
  (`self.ActivateAbilityNoTarget` AbilitySlot AbilityOwner))

(event `ServerSendTraceUnitToAbility`
  (params (AbilityOwner :type "AP_FightUnit Object Reference") (AbilitySlot :type Integer) (Start :type "Vector Structure") (Direction :type "Vector Structure"))
  (`self.SendLineTraceUnitToAbility` AbilityOwner AbilitySlot Start Direction))

(event `ServerLevelUpAbility`
  (params (AbilitySlot :type Integer))
  (`AP_FightUnit.LevelUpAbility` (`self.LeaderUnit`) AbilitySlot))

(event `BuyItem`
  (params (Slot :type Integer))
  (`self.IfPawnValid`
    (:`Is Valid`
      (bind (_itemuser _itemseller) (`self.FindShop`)
        (:`Is Valid`
          (`ItemUser.BuyItem` _itemuser _itemseller Slot))))))

(event `SellItem`)

(event `EquipItem`
  (params (Slot :type Integer))
  (`self.IfPawnValid`
    (:`Is Valid`
      (`ItemUser.EquipItem` (`AP_FightUnit.ItemUser` (`self.LeaderUnit`)) Slot))))

(event `UnequipItem`
  (params (Slot :type Integer))
  (`self.IfPawnValid`
    (:`Is Valid`
      (`ItemUser.UnequipItem` (`AP_FightUnit.ItemUser` (`self.LeaderUnit`)) Slot))))

(event `CheatGiveXP`
  (`AP_AttributeSet.GiveExp` (`AP_FightUnit.Stats` (`self.LeaderUnit`)) 200.0))

(fn `ActivateAbilityNoTarget`
  (params (AbilitySlot :type Integer) (AbilityOwner :type "AP_FightUnit Object Reference"))
  (`AbilityUser.ActivateAbility` (`AP_FightUnit.AbilityUser` AbilityOwner) AbilitySlot))

(fn `CancelTargeting`
  (set `self.TargetMode` "None")
  (`self.UpdateMouseCursor`))

(fn `CheckUnitValidity`
  (`/Engine/EditorBlueprintResources/StandardMacros.IsValid` (`self.LeaderUnit`)
    (:`Is Valid`
      (`self.OnPawnChanged` (`self.LeaderUnit`))
      (`self.EnableInput` self))
    (:`Is Not Valid`
      (`self.DisableInput` self))))

(fn `ConfirmTargeting`
  (params (AbilitySlot :type Integer) (RayStart :type "Vector Structure") (RayDirection :type "Vector Structure"))
  (locals (IsComboAbility :type Boolean) (IsInProgress :type Boolean) (Ability :type "AP_AbilityBase Object Reference") (State :type "EAbilityState Enum" :default "Ready"))
  (set `local.Ability` (`self.GetAbility` (`local.AbilitySlot`)))
  (set `local.State` (`self.GetAbilityState` (`local.AbilitySlot`)))
  (if (and (`|EnumEquality` (`AP_AbilityBase.ActivatingPolicy` (`local.Ability`)) "ActiveCombo") (`|EnumEquality` (`local.State`) "Casting"))
    (`self.ServerActivateAbilityNoTarget` (`local.AbilitySlot`) (`self.LeaderUnit`) :!label _label)
    (`self.ClearTarget` :!label _label_2)
    (`self.SetTargetingMode` "None")
    (else
      (switch `ETargetingPolicy` (`AP_AbilityBase.TargetingPolicy` (`local.Ability`))
        (:`None`
          (goto _label))
        (:`Ground`
          (bind (_outlocation _returnvalue) (`AP_FightUnit.LineTraceGround` (`self.LeaderUnit`) (`local.RayStart`) (`local.RayDirection`)))
          (if _returnvalue
            (`self.WriteLocationTarget` _outlocation (`local.AbilitySlot`)
              (:`Out`
                _)))
          (`self.ServerSendTargetToAbility` (`self.TargetUnit`) (`self.TargetLocation`) (`self.GetAbility` (`local.AbilitySlot`)) (`self.LeaderUnit`) :!label _label_3)
          (goto _label_2))
        (:`UnitAll`
          (bind (_outactor _returnvalue_2) (`AP_FightUnit.LineTraceUnitAuto` (`self.LeaderUnit`) (`AP_AbilityBase.TargetingPolicy` (`local.Ability`)) (`local.RayStart`) (`local.RayDirection`) :!label _label_4))
          (if _returnvalue_2
            (`self.WriteUnitTarget` _outactor (`local.AbilitySlot`)
              (:`Out`
                (goto _label_3)))))
        (:`UnitExcludeSelf`
          (goto _label_4))
        (:`UnitAlly`
          (goto _label_4))
        (:`UnitAllyExcludeSelf`
          (goto _label_4))
        (:`UnitEnemy`
          (goto _label_4))))))

(fn `EnterTargeting`
  (params (AbilitySlot :type Integer))
  (bind _ability (`self.GetAbility` (`local.AbilitySlot`)))
  (set `self.TargetAbility` AbilitySlot)
  (`self.IfPawnValid`
    (:`Is Valid`
      (switch `EActivatingPolicy` (`AP_AbilityBase.ActivatingPolicy` _ability)
        (:`Toggle`
          (`self.ServerActivateAbilityNoTarget` (`local.AbilitySlot`) (`self.LeaderUnit`) :!label _label)
          (`self.CancelTargeting`))
        (:`Active`
          (switch `ETargetingPolicy` (`AP_AbilityBase.TargetingPolicy` _ability) :!label _label_2
            (:`None`
              (goto _label))
            (:`Ground`
              _)
            (:`UnitAll`
              _)
            (:`UnitExcludeSelf`
              _)
            (:`UnitAlly`
              _)
            (:`UnitAllyExcludeSelf`
              _)
            (:`UnitEnemy`
              _))
          (`KismetSystemLibrary.PrintString` "enter targeting")
          (`self.SetTargetingMode` (`AP_AbilityBase.TargetingPolicy` (`self.GetAbility` (`local.AbilitySlot`)))))
        (:`ActiveAutocast`
          (goto _label_2))
        (:`ActiveCombo`
          (goto _label_2))))))

(fn `OnRep_LeaderUnit`
  (`self.CheckUnitValidity`))

(fn `RetrieveControlledPawn`
  (bind _asap_fight_unit (cast `AP_FightUnit` (`self.K2_GetPawn`))
    (:`then`
      (set `self.LeaderUnit` _asap_fight_unit))
    (:`CastFailed`
      (set `self.LeaderUnit` null)))
  (`self.CheckUnitValidity`))

(fn `Send Target to Ability`
  (params (Actor :type "Actor Object Reference") (Location :type "Vector Structure") (Ability :type "AP_AbilityBase Object Reference") (AbilityOwner :type "Actor Object Reference"))
  (bind _returnvalue (`AbilitySystemBlueprintLibrary.AbilityTargetDataFromActor` (`local.Actor`)))
  (`AbilitySystemBlueprintLibrary.SendGameplayEventToActor` (`local.AbilityOwner`) (struct :`TagName` "Combat.Trigger_Ability_By_Controller") (make `GameplayEventData` :`OptionalObject` (`local.Ability`) :`TargetData` (select `ETargetingPolicy` (`AP_AbilityBase.TargetingPolicy` (`local.Ability`)) :`Ground` (`AbilitySystemBlueprintLibrary.AbilityTargetDataFromLocations` (make `GameplayAbilityTargetingLocationInfo` :`LiteralTransform` (`self.GetTransform` (`local.AbilityOwner`))) (make `GameplayAbilityTargetingLocationInfo` :`LiteralTransform` (`KismetMathLibrary.Conv_VectorToTransform` (`local.Location`)))) :`UnitAll` _returnvalue :`UnitExcludeSelf` _returnvalue :`UnitAlly` _returnvalue :`UnitAllyExcludeSelf` _returnvalue :`UnitEnemy` _returnvalue))))

(fn `SendLineTraceGroundToAbility`
  (params (AbilityOwner :type "AP_FightUnit Object Reference") (AbilitySlot :type Integer) (Start :type "Vector Structure") (Direction :type "Vector Structure"))
  (bind (_outlocation _returnvalue) (`AP_FightUnit.LineTraceGround` AbilityOwner Start Direction))
  (if _returnvalue
    (`self.Send Target to Ability` null _outlocation (`AbilityUser.GetAbility` (`AP_FightUnit.AbilityUser` AbilityOwner) AbilitySlot) (`local.AbilityOwner`))))

(fn `SendLineTraceUnitToAbility`
  (params (AbilityOwner :type "AP_FightUnit Object Reference") (AbilitySlot :type Integer) (Start :type "Vector Structure") (Direction :type "Vector Structure"))
  (bind _returnvalue (`AbilityUser.GetAbility` (`AP_FightUnit.AbilityUser` AbilityOwner) AbilitySlot))
  (bind (_outactor _returnvalue_2) (`AP_FightUnit.LineTraceUnitAuto` AbilityOwner (`AP_AbilityBase.TargetingPolicy` _returnvalue) Start Direction))
  (if _returnvalue_2
    (`self.Send Target to Ability` _outactor (0.0 0.0 0.0) _returnvalue (`local.AbilityOwner`))))

(fn `UserConstructionScript`)
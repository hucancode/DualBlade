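; RTS player controller for commanding multiple units: camera panning, HUD click selection, move, stop, hold and ability orders.
; Ability keys request a server eligibility check, then either enter crosshair targeting or cast directly.
; Orders become AI Blackboard writes; basic attacks apply to all selected units, other targeted skills only to the leader.
; Unit targeting picks trace channels from skill policy and team, skipping units hidden from the team.
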(event `InputAxis|CameraX`
  (params (AxisValue :type "Float (single-precision)"))
  (bind _returnvalue (`self.K2_GetPawn`))
  (`/Engine/EditorBlueprintResources/StandardMacros.IsValid` _returnvalue
    (:`Is Valid`
      (`Pawn.AddMovementInput` _returnvalue (`SceneComponent.GetRightVector` (`Actor.RootComponent` _returnvalue)) AxisValue false))))

(event `InputAxis|CameraY`
  (params (AxisValue :type "Float (single-precision)"))
  (bind _returnvalue (`self.K2_GetPawn`))
  (`/Engine/EditorBlueprintResources/StandardMacros.IsValid` _returnvalue
    (:`Is Valid`
      (`Pawn.AddMovementInput` _returnvalue (`SceneComponent.GetForwardVector` (`Actor.RootComponent` _returnvalue)) AxisValue false))))

(event `InputAction|CancelTargeting`
  (params (Key :type "Key Structure"))
  (:`Pressed`
    (if (`self.Targeting`)
      (`self.CancelTargeting`)
      (else
        (`self.Move`)))))

(event `InputAction|ConfirmTargeting`
  (params (Key :type "Key Structure"))
  (bind (_worldlocation _worlddirection) (`self.DeprojectMousePositionToWorld`))
  (bind _targeting (`self.Targeting`))
  (:`Pressed`
    (if (not _targeting)
      (bind _asrts_hud (cast `/Game/Common/UI/RTS_HUD` (`self.GetHUD`)))
      (`/Game/Common/UI/RTS_HUD.MouseClicked` _asrts_hud null Key)))
  (:`Released`
    (if _targeting
      (`self.ServerConfirmTargeting` (`self.ControlledUnits`) (`.LeaderUnit` (`self.LeaderUnit`)) (`self.TargetingAbility`) _worldlocation _worlddirection)
      (else
        (bind _asrts_hud_2 (cast `/Game/Common/UI/RTS_HUD` (`self.GetHUD`)))
        (`/Game/Common/UI/RTS_HUD.MouseReleased` _asrts_hud_2 null Key)))))

(event `InputAction|WeaponAbility`
  (params (Key :type "Key Structure"))
  (:`Pressed`
    (`self.ActivateAbility` 0)))

(event `InputAction|UseAbility1`
  (params (Key :type "Key Structure"))
  (:`Pressed`
    (`self.ActivateAbility` 1)))

(event `InputAction|UseAbility2`
  (params (Key :type "Key Structure"))
  (:`Pressed`
    (`self.ActivateAbility` 2)))

(event `InputAction|UseAbility3`
  (params (Key :type "Key Structure"))
  (:`Pressed`
    (`self.ActivateAbility` 3)))

(event `InputAction|UseAbility4`
  (params (Key :type "Key Structure"))
  (:`Pressed`
    (`self.ActivateAbility` 4)))

(event `InputAction|UseAbility5`
  (params (Key :type "Key Structure"))
  (:`Pressed`
    (`self.ActivateAbility` 5)))

(event `InputAction|UseAbility6`
  (params (Key :type "Key Structure"))
  (:`Pressed`
    (`self.ActivateAbility` 6)))

(event `InputAction|Hold`
  (params (Key :type "Key Structure"))
  (:`Pressed`
    (`self.Hold`)))

(event `InputAction|Stop`
  (params (Key :type "Key Structure"))
  (:`Pressed`
    (`self.Stop`)))

(event `ActivateAbility`
  (params (AbilitySlot :type Integer))
  (set `self.TargetingAbility` AbilitySlot)
  (`self.ServerEnterTargeting` (`.LeaderUnit` (`self.LeaderUnit`)) (`self.TargetingAbility`)))

(event `ServerEnterTargeting`
  (params (Unit :type "Object Object Reference") (AbilitySlot :type Integer))
  (`self.EnterTargeting` Unit AbilitySlot))

(event `ServerConfirmTargeting`
  (params (AllUnits :type "Array of Actor Object Reference (by ref)") (Leader :type "Object Object Reference") (AbilitySlot :type Integer) (RayStart :type "Vector Structure") (RayDirection :type "Vector Structure"))
  (`self.ConfirmTargeting` AllUnits Leader AbilitySlot RayStart RayDirection))

(event `ClientEnterTargeting`
  (set `self.Targeting` true)
  (set `self.CurrentMouseCursor` (select `bool` (`self.Targeting`) :`false` "Default" :`true` "Crosshairs" :!type "EMouseCursor Enum") :!label _label))

(event `ClientConfirmTargeting`
  (set `self.Targeting` false)
  (goto _label))

(event `ServerWriteTargetLocation`
  (params (Unit :type "Actor Object Reference") (Location :type "Vector Structure"))
  (`BlackboardComponent.SetValueAsVector` (`AIBlueprintHelperLibrary.GetBlackboard` Unit) (`self.TargetLocation_KeyName`) Location))

(event `ServerWriteAIState`
  (params (Unit :type "Actor Object Reference") (State :type "/Game/Common/AI/AI_BasicState Enum" :default "NewEnumerator0"))
  (`BlackboardComponent.SetValueAsEnum` (`AIBlueprintHelperLibrary.GetBlackboard` Unit) (`self.AIState_KeyName`) State))

(event `ServerWriteActorTarget`
  (params (Target :type "Actor Object Reference") (Unit :type "Actor Object Reference"))
  (bind _returnvalue (`AIBlueprintHelperLibrary.GetBlackboard` Unit))
  (bind _targetactor_keyname (`self.TargetActor_KeyName`))
  (`/Engine/EditorBlueprintResources/StandardMacros.IsValid` Target
    (:`Is Valid`
      (`BlackboardComponent.SetValueAsObject` _returnvalue _targetactor_keyname Target))
    (:`Is Not Valid`
      (`BlackboardComponent.ClearValue` _returnvalue _targetactor_keyname))))

(event `ServerWriteSkillToCast`
  (params (Unit :type "Actor Object Reference") (Slot :type Integer))
  (bind _returnvalue (`AIBlueprintHelperLibrary.GetBlackboard` Unit))
  (bind _castrange_keyname (`self.CastRange_KeyName`))
  (bind _asap_hero (cast `` Unit))
  (`BlackboardComponent.SetValueAsInt` _returnvalue (`self.SkillToCast_KeyName`) Slot)
  (bind _returnvalue_2 (`self.GetAbility` _asap_hero Slot))
  (bind _asground_target_skill (cast `/Game/AgeOfDualBlade/Abilities/Core/Base/Ground_Target_Skill` _returnvalue_2)
    (:`then`
      (bind _result (`/Game/AgeOfDualBlade/Abilities/Core/Base/Ground_Target_Skill.GetCastRange` _asground_target_skill))
      (`BlackboardComponent.SetValueAsFloat` _returnvalue _castrange_keyname _result))
    (:`CastFailed`
      (bind _asunit_target_skill (cast `/Game/AgeOfDualBlade/Abilities/Core/Base/Unit_Target_Skill` _returnvalue_2))
      (bind _result_2 (`/Game/AgeOfDualBlade/Abilities/Core/Base/Unit_Target_Skill.GetCastRange` _asunit_target_skill))
      (`BlackboardComponent.SetValueAsFloat` _returnvalue _castrange_keyname _result_2))))

(event `ServerClearTarget`
  (params (Unit :type "Actor Object Reference"))
  (bind _returnvalue (`AIBlueprintHelperLibrary.GetBlackboard` Unit))
  (`BlackboardComponent.SetValueAsInt` _returnvalue (`self.SkillToCast_KeyName`) -1)
  (`BlackboardComponent.ClearValue` _returnvalue (`self.TargetActor_KeyName`))
  (`BlackboardComponent.SetValueAsFloat` _returnvalue (`self.CastRange_KeyName`) 99999.0)
  (`BlackboardComponent.ClearValue` _returnvalue (`self.TargetLocation_KeyName`)))

(event `Key|One`
  (params (Key :type "Key Structure"))
  (:`Pressed`
    (`self.SetTeam1`)
    (`KismetSystemLibrary.PrintString` "set team 1")))

(event `Key|Two`
  (params (Key :type "Key Structure"))
  (:`Pressed`
    (`self.SetTeam2`)
    (`KismetSystemLibrary.PrintString` "set team 2")))

(event `Key|V`
  (params (Key :type "Key Structure")))

(event `Key|B`
  (params (Key :type "Key Structure")))

(event `RetrievePlayerInfo`
  (bind _asgame_info_instance (cast `/Game/Common/GameMode/GameInfoInstance` (`GameplayStatics.GetGameInstance`)))
  (bind _lobbypc (`/Game/Common/GameMode/GameInfoInstance.LobbyPC` _asgame_info_instance))
  (`KismetSystemLibrary.PrintString` (`KismetStringLibrary.Concat_StrStr` (`KismetSystemLibrary.GetDisplayName` _lobbypc) " - " (`KismetSystemLibrary.GetDisplayName` self) " client retrieve player info") true true (struct :`G` 0.200763 :`B` 1.0 :`A` 1.0))
  (`self.SubmitPlayerInfo` _lobbypc self))

(event `SubmitPlayerInfo`
  (params (LobbyPC :type "/Game/Common/GameMode/LobbyPC Object Reference") (ActionPC :type "/Game/Common/GameMode/BP_Multi_Unit_Controller Object Reference"))
  (bind _asaction_game_mode (cast `/Game/Common/GameMode/ActionGameMode` (`GameplayStatics.GetGameMode`)))
  (`KismetSystemLibrary.PrintString` "server submit player info" true true (struct :`R` 0.348067 :`G` 1.0 :`B` 0.480089 :`A` 1.0))
  (`/Game/Common/GameMode/ActionGameMode.SubmitPlayerInfo` _asaction_game_mode LobbyPC ActionPC))

(event `self.ReceiveBeginPlay`
  (`KismetSystemLibrary.PrintString` "player controller -> begin play" true true (struct :`G` 0.200763 :`B` 1.0 :`A` 1.0))
  (`self.RetrievePlayerInfo`))

(fn `CancelTargeting`
  (set `self.Targeting` false)
  (set `self.CurrentMouseCursor` "Default"))

(fn `ConfirmTargeting`
  (params (AllUnits :type "Array of Actor Object Reference") (Leader :type "Object Object Reference") (AbilitySlot :type Integer) (RayStart :type "Vector Structure") (RayDirection :type "Vector Structure"))
  (locals (IsUnitTarget :type Boolean) (IsGroundTarget :type Boolean) (IsBasicAttack :type Boolean))
  (bind _returnvalue (`GameplayStatics.GetObjectClass` (`self.GetAbility` (`.Leader` (`local.Leader`)) (`local.AbilitySlot`))))
  (bind _output_get (set `local.IsBasicAttack` (== (`local.AbilitySlot`) 0)))
  (if _output_get
    (bind (_hit _actor) (`self.RayHitTestUnit` (`local.RayStart`) (`local.RayDirection`)))
    (if _hit
      (for _array_element (`local.AllUnits`)
        (`self.ServerClearTarget` _array_element)
        (`self.ServerWriteActorTarget` _actor _array_element)
        (`self.ServerWriteSkillToCast` _array_element (`local.AbilitySlot`))
        (`self.ServerWriteAIState` _array_element "NewEnumerator7")
        (`self.StopAllMontage` _array_element))
      (`self.ClientConfirmTargeting`)
      (else
        (bind (_hit_2 _location) (`self.RayHitTestFloor` (`local.RayStart`) (`local.RayDirection`)))
        (if _hit_2
          (for _array_element_2 (`local.AllUnits`)
            (`self.ServerClearTarget` _array_element_2)
            (`self.ServerWriteTargetLocation` _array_element_2 _location)
            (`self.ServerWriteSkillToCast` _array_element_2 (`local.AbilitySlot`))
            (`self.ServerWriteAIState` _array_element_2 "NewEnumerator6")
            (`self.StopAllMontage` _array_element_2))
          (`self.ClientConfirmTargeting`))))
    (elif (`KismetMathLibrary.ClassIsChildOf` _returnvalue "/Game/AgeOfDualBlade/Abilities/Core/Base/Unit_Target_Skill.Unit_Target_Skill_C")
      (bind (_hit_3 _actor_2) (`self.RayHitTestUnit` (`local.RayStart`) (`local.RayDirection`)))
      (if _hit_3
        (`self.ServerClearTarget` (`.Leader` (`local.Leader`)))
        (`self.ServerWriteActorTarget` _actor_2 (`.Leader` (`local.Leader`)))
        (`self.ServerWriteSkillToCast` (`.Leader` (`local.Leader`)) (`local.AbilitySlot`) :!label _label)
        (`self.ServerWriteAIState` (`.Leader` (`local.Leader`)) "NewEnumerator3")
        (`Character.StopAnimMontage` (`.Leader` (`local.Leader`)) null)
        (`self.ClientConfirmTargeting`))
      (elif (`KismetMathLibrary.ClassIsChildOf` _returnvalue "/Game/AgeOfDualBlade/Abilities/Core/Base/Ground_Target_Skill.Ground_Target_Skill_C")
        (bind (_hit_4 _location_2) (`self.RayHitTestFloor` (`local.RayStart`) (`local.RayDirection`)))
        (if _hit_4
          (`self.ServerClearTarget` (`.Leader` (`local.Leader`)))
          (`self.ServerWriteTargetLocation` (`.Leader` (`local.Leader`)) _location_2)
          (goto _label))))))

(fn `EnterTargeting`
  (params (Unit :type "Object Object Reference") (AbilitySlot :type Integer))
  (locals (IsGroundTarget :type Boolean) (IsUnitTarget :type Boolean))
  (`KismetSystemLibrary.PrintString` (`KismetStringLibrary.Concat_StrStr` "server check for ability eligibity" (`KismetSystemLibrary.GetDisplayName` Unit) (`KismetStringLibrary.Conv_IntToString` AbilitySlot)))
  (`/Engine/EditorBlueprintResources/StandardMacros.IsValid` Unit
    (:`Is Valid`
      (if (`self.CanActivateAbility` Unit AbilitySlot)
        (bind _result (`self.GetAbilityInfo` Unit AbilitySlot))
        (bind _returnvalue (`GameplayStatics.GetObjectClass` _result))
        (set `local.IsUnitTarget` (`KismetMathLibrary.ClassIsChildOf` _returnvalue "/Game/AgeOfDualBlade/Abilities/Core/Base/Unit_Target_Skill.Unit_Target_Skill_C"))
        (set `local.IsGroundTarget` (`KismetMathLibrary.ClassIsChildOf` _returnvalue "/Game/AgeOfDualBlade/Abilities/Core/Base/Ground_Target_Skill.Ground_Target_Skill_C"))
        (if (or (`local.IsUnitTarget`) (`local.IsGroundTarget`))
          (`KismetSystemLibrary.PrintString` "enter targeting")
          (`self.ClientEnterTargeting`)
          (else
            (`KismetSystemLibrary.PrintString` (`KismetStringLibrary.Concat_StrStr` "this skill is, " (`KismetSystemLibrary.GetClassDisplayName` (`GameplayStatics.GetObjectClass` _result)) ", not unit target, not ground target, so skip targeting phase" (`KismetStringLibrary.Conv_IntToString` (`self.TargetingAbility`))))
            (`KismetSystemLibrary.PrintString` "activate skill directly")
            (`self.ActivateAbility` (`.Unit` (`local.Unit`)) (`local.AbilitySlot`))))))))

(fn `GetAbilityInfo`
  (params (Unit :type "Object Object Reference") (AbilitySlot :type Integer))
  (returns (Result :type "GameplayAbility Object Reference"))
  (bind _returnvalue (`self.GetAbility` Unit AbilitySlot))
  (`/Engine/EditorBlueprintResources/StandardMacros.IsValid` _returnvalue
    (:`Is Valid`
      (return _returnvalue))
    (:`Is Not Valid`
      (return null))))

(fn `Hold`
  (for _array_element (`self.ControlledUnits`)
    (`self.ServerClearTarget` _array_element)
    (`BlackboardComponent.SetValueAsEnum` (`AIBlueprintHelperLibrary.GetBlackboard` _array_element) (`self.AIState_KeyName`) (enumliteral `/Game/Common/AI/AI_BasicState` "NewEnumerator1"))))

(fn `MarkAllUnitSelected`
  (params (Selected :type Boolean))
  (for _array_element (`self.ControlledUnits`)
    (bind _asap_hero (cast `` _array_element))
    (`self.SelectHero` _asap_hero Selected)))

(fn `MouseHitTestFloor`
  (returns (Hit :type Boolean) (Location :type "Vector Structure"))
  (bind (_hitresult _returnvalue) (`self.GetHitResultUnderCursorByChannel` "TraceTypeQuery3" false))
  (return _returnvalue (`.Location` (`GameplayStatics.BreakHitResult` _hitresult))))

(fn `MouseHitTestUnit`
  (returns (Hit :type Boolean) (Actor :type "Actor Object Reference"))
  (bind (_hitresult _returnvalue) (`self.GetHitResultUnderCursorByChannel` "TraceTypeQuery11" false))
  (return _returnvalue (`.HitActor` (`GameplayStatics.BreakHitResult` _hitresult))))

(fn `Move`
  (bind (_hit _location) (`self.MouseHitTestFloor`))
  (if _hit
    (for _array_element (`self.ControlledUnits`)
      (bind _ascharacter (cast `Character` _array_element))
      (`self.StopAllMontage` _ascharacter)
      (`self.ServerClearTarget` _array_element)
      (`GameplayStatics.SpawnEmitterAtLocation` "/Game/LinhiBlade/MouseClickParticle/P_MouseClick.P_MouseClick" _location (struct :`Roll` 90.0) (1.0 1.0 1.0) true "AutoRelease")
      (`self.ServerWriteTargetLocation` _array_element _location)
      (`self.ServerWriteAIState` _array_element "NewEnumerator5"))))

(fn `RayHitTestFloor`
  (params (Start :type "Vector Structure") (Direction :type "Vector Structure"))
  (returns (Hit :type Boolean) (Location :type "Vector Structure"))
  (bind (_outhit _returnvalue) (`KismetSystemLibrary.LineTraceSingle` Start (* Direction 200000.0) "TraceTypeQuery3"))
  (return _returnvalue (`.Location` (`GameplayStatics.BreakHitResult` _outhit))))

(fn `RayHitTestUnit`
  (params (Start :type "Vector Structure") (Direction :type "Vector Structure"))
  (returns (Hit :type Boolean) (Actor :type "Actor Object Reference"))
  (locals (HitActor :type "Actor Object Reference"))
  (bind _result (`self.GetAbilityInfo` (`.LeaderUnit` (`self.LeaderUnit`)) (`self.TargetingAbility`)))
  (bind _asap_skill_base (cast `/Game/AgeOfDualBlade/Abilities/Core/Base/AP_Skill_Base` _result))
  (bind _returnvalue (`self.GetTeam` (`.LeaderUnit` (`self.LeaderUnit`))))
  (bind (_outhits _returnvalue_2) (`KismetSystemLibrary.LineTraceMulti` :`Start` Start :`End` (* Direction 200000.0) :`TraceChannel` (select `/Game/AgeOfDualBlade/Abilities/Core/Base/ETargetingPolicy` (`/Game/AgeOfDualBlade/Abilities/Core/Base/AP_Skill_Base.TargetingPolicy` _asap_skill_base) :`NewEnumerator13` "TraceTypeQuery11" :`NewEnumerator11` (select `EGameTeam` _returnvalue :`Neutral` "TraceTypeQuery10" :`Team1` "TraceTypeQuery8" :`Team2` "TraceTypeQuery9" :`NoTeam` "TraceTypeQuery1" :!type "ETraceTypeQuery Enum") :`NewEnumerator12` (select `EGameTeam` _returnvalue :`Neutral` "TraceTypeQuery3" :`Team1` "TraceTypeQuery9" :`Team2` "TraceTypeQuery8" :`NoTeam` "TraceTypeQuery1" :!type "ETraceTypeQuery Enum") :`NewEnumerator7` "TraceTypeQuery7" :`NewEnumerator1` (select `EGameTeam` _returnvalue :`Neutral` "TraceTypeQuery6" :`Team1` "TraceTypeQuery4" :`Team2` "TraceTypeQuery5" :`NoTeam` "TraceTypeQuery1" :!type "ETraceTypeQuery Enum") :`NewEnumerator3` (select `EGameTeam` _returnvalue :`Neutral` "TraceTypeQuery3" :`Team1` "TraceTypeQuery5" :`Team2` "TraceTypeQuery4" :`NoTeam` "TraceTypeQuery1" :!type "ETraceTypeQuery Enum")) :`bIgnoreSelf` false))
  (if _returnvalue_2
    (for _array_element _outhits
      (bind (_bblockinghit _binitialoverlap _time _distance _location _impactpoint _normal _impactnormal _physmat _hitactor) (`GameplayStatics.BreakHitResult` _array_element))
      (bind _asap_hero (cast `` _hitactor))
      (bind _returnvalue_3 (`self.IsVisibleToTeam` :`self` _asap_hero))
      (if _returnvalue_3
        (set `local.HitActor` _hitactor)
        (break)))
    (`/Engine/EditorBlueprintResources/StandardMacros.IsValid` (`local.HitActor`)
      (:`Is Valid`
        (return true (`local.HitActor`)))
      (:`Is Not Valid`
        (return false null)))
    (else
      (return false null))))

(fn `SelectUnits`
  (params (Units :type "Array of Actor Object Reference"))
  (`self.MarkAllUnitSelected` false)
  (set `self.ControlledUnits` Units)
  (bind (_arrayindex _arrayelement) (`/Engine/EditorBlueprintResources/StandardMacros.ReverseForEachLoop` (`self.ControlledUnits`))
    (:`LoopBody`
      (bind _asap_hero (cast `` _arrayelement))
      (bind _returnvalue (`self.IsLogicalController` _asap_hero self))
      (if (not (and (not (`self.IsDead` _asap_hero)) _returnvalue))
        (`KismetArrayLibrary.Array_Remove` (`self.ControlledUnits`) _arrayindex)))
    (:`Completed`
      (`self.MarkAllUnitSelected` true)
      (set `self.LeaderUnit` null)
      (for _array_element (`self.ControlledUnits`)
        (bind _asap_hero_2 (cast `` _array_element))
        (bind (_output_get _output_get_2) (set `self.LeaderUnit` null _asap_hero_2))
        (`self.OnControlledUnitChanged` _output_get_2)
        (break)))))

(fn `SetTeam1`)

(fn `SetTeam2`)

(fn `Stop`
  (for _array_element (`self.ControlledUnits`)
    (bind _ascharacter (cast `Character` _array_element))
    (`Character.StopAnimMontage` _ascharacter null)
    (`self.ServerClearTarget` _array_element)
    (`BlackboardComponent.SetValueAsEnum` (`AIBlueprintHelperLibrary.GetBlackboard` _array_element) (`self.AIState_KeyName`) (enumliteral `/Game/Common/AI/AI_BasicState` "NewEnumerator1"))))

(fn `StopAllMontage`
  (params (Unit :type "Actor Object Reference"))
  (bind _ascharacter (cast `Character` Unit))
  (`Character.StopAnimMontage` _ascharacter null))

(fn `UserConstructionScript`)
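; AI Controller for a "camper" AI that runs the BT_CamperMaster behavior tree and manages its auto-target.
; On BeginPlay it starts the tree, resets skill, state and cast range blackboard keys, and stores the pawn's starting location.
; On perception updates it keeps the blackboard target while currently perceived, otherwise replacing it with a random actor from the perceived list, or none if empty.
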(event `self.ReceiveBeginPlay`
  (bind _returnvalue (`self.K2_GetPawn`))
  (`self.RunBehaviorTree` "/Game/Common/AI/BT_CamperMaster.BT_CamperMaster")
  (`self.ResetBB`)
  (`BlackboardComponent.SetValueAsVector` (`AIBlueprintHelperLibrary.GetBlackboard` _returnvalue) (`self.Location_KeyName`) (`self.K2_GetActorLocation` _returnvalue)))

(event `self.AIPerception.OnPerceptionUpdated`
  (params (UpdatedActors :type "Array of Actor Object Reference (by ref)"))
  (bind _result (`self.GetCurrentTarget`))
  (`/Engine/EditorBlueprintResources/StandardMacros.IsValid` _result
    (:`Is Valid`
      (bind _returnvalue (`self.IsInPerceivedList` _result))
      (if (not _returnvalue)
        (bind _result_2 (`self.GetRandomTarget` :!label _label))
        (`self.SetCurrentTarget` _result_2)))
    (:`Is Not Valid`
      (goto _label))))

(fn `GetCurrentTarget`
  (returns (Result :type "Actor Object Reference"))
  (bind _asactor (cast `Actor` (`BlackboardComponent.GetValueAsObject` (`AIBlueprintHelperLibrary.GetBlackboard` (`self.K2_GetPawn`)) (`self.AutoTargetActor_KeyName`)))
    (:`then`
      (return _asactor))
    (:`CastFailed`
      (return null))))

(fn `GetRandomTarget`
  (returns (Result :type "Actor Object Reference"))
  (bind _outactors (`AIPerceptionComponent.GetPerceivedActors` (`self.AIPerception`) null))
  (bind _returnvalue (`KismetArrayLibrary.Array_Length` _outactors))
  (if (> _returnvalue 0)
    (return (`|GetArrayItem` _outactors (`KismetMathLibrary.RandomInteger` _returnvalue)))
    (else
      (return null))))

(fn `IsInPerceivedList`
  (params (ItemToFind :type "Actor Object Reference (by ref)"))
  (returns (ReturnValue :type Boolean))
  (return (>= (`KismetArrayLibrary.Array_Find` (`AIPerceptionComponent.GetCurrentlyPerceivedActors` (`self.AIPerception`) null) ItemToFind) 0)))

(fn `ResetBB`
  (bind _returnvalue (`AIBlueprintHelperLibrary.GetBlackboard` (`self.K2_GetPawn`)))
  (`BlackboardComponent.SetValueAsInt` _returnvalue (`self.SkillToCast_KeyName`) -1)
  (`BlackboardComponent.SetValueAsEnum` _returnvalue (`self.CurrentState_KeyName`) (enumliteral `/Game/Common/AI/AI_BasicState` "NewEnumerator0"))
  (`BlackboardComponent.SetValueAsFloat` _returnvalue (`self.CastRange_KeyName`) 100000.0))

(fn `SetCurrentTarget`
  (params (NewTarget :type "Actor Object Reference"))
  (`BlackboardComponent.SetValueAsObject` (`AIBlueprintHelperLibrary.GetBlackboard` (`self.K2_GetPawn`)) (`self.AutoTargetActor_KeyName`) NewTarget))

(fn `UserConstructionScript`)
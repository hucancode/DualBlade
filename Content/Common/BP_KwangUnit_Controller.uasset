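; Player controller for RTS-style hero control that pans the camera pawn and issues orders to a selected hero unit.
; Clicking line-traces to select an AP_Hero; move and attack-move orders send the cursor hit location to the unit's AI controller.
; Ability inputs call SpellAttack by slot and track the unit's targeting state, which confirm and cancel inputs resolve through its Ability System Component.
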(event `InputAxis|CameraX`
  (params (AxisValue :type "Float (single-precision)"))
  (bind _returnvalue (`self.K2_GetPawn`))
  (`Pawn.AddMovementInput` _returnvalue (`SceneComponent.GetRightVector` (`Actor.RootComponent` _returnvalue)) AxisValue false))

(event `self.ReceiveBeginPlay`)

(event `InputAxis|CameraY`
  (params (AxisValue :type "Float (single-precision)"))
  (bind _returnvalue (`self.K2_GetPawn`))
  (`Pawn.AddMovementInput` _returnvalue (`SceneComponent.GetForwardVector` (`Actor.RootComponent` _returnvalue)) AxisValue false))

(event `self.ReceiveTick`
  (params (DeltaSeconds :type "Float (single-precision)")))

(event `InputAction|MoveHold`
  (params (Key :type "Key Structure"))
  (bind (_hitresult _returnvalue) (`self.GetHitResultUnderCursorByChannel` "TraceTypeQuery3" false))
  (bind _controlledunit (`self.ControlledUnit`))
  (bind (_bblockinghit _binitialoverlap _time _distance _location) (`GameplayStatics.BreakHitResult` _hitresult))
  (:`Pressed`
    (if (`AP_Hero.IsTargeting` (`self.ControlledUnit`))
      (`KismetSystemLibrary.PrintString` "targeting")
      (elif _returnvalue
        (`/Engine/EditorBlueprintResources/StandardMacros.IsValid` _controlledunit
          (:`Is Valid`
            (bind _asaicontroller (cast `AIController` (`Pawn.GetController` _controlledunit))
              (:`then`
                (`Character.StopAnimMontage` _controlledunit null)
                (`AIController.MoveToLocation` _asaicontroller _location 1.0 true true false true null true)
                (`GameplayStatics.SpawnEmitterAtLocation` "/Game/LinhiBlade/MouseClickParticle/P_MouseClick.P_MouseClick" _location (struct :`Roll` 90.0) (1.0 1.0 1.0) true "AutoRelease"))
              (:`CastFailed`
                (`KismetSystemLibrary.PrintString` "controller is not an AIController"))))
          (:`Is Not Valid`
            (`KismetSystemLibrary.PrintString` "controlled unit not valid")))
        (else
          (`KismetSystemLibrary.PrintString` "hit failed"))))))

(event `Key|M`
  (params (Key :type "Key Structure"))
  (:`Released`
    (`KismetSystemLibrary.PrintString` "M pressed")
    (bind _asac_basic (cast `/Game/Common/AI/AC_Basic` (`AIBlueprintHelperLibrary.GetAIController` (`self.ControlledUnit`))))
    (`/Game/Common/AI/AC_Basic.AttackMove` _asac_basic (`.Location` (`GameplayStatics.BreakHitResult` (`self.GetHitResultUnderCursorByChannel` "TraceTypeQuery3" false))))))

(event `InputAction|WeaponAbility`
  (params (Key :type "Key Structure"))
  (:`Pressed`
    (`self.SpellAttack` 0)))

(event `InputAction|ConfirmAbility`
  (params (Key :type "Key Structure"))
  (bind _controlledunit (`self.ControlledUnit`))
  (:`Pressed`
    (if (`self.Targeting`)
      (`/Engine/EditorBlueprintResources/StandardMacros.IsValid` _controlledunit
        (:`Is Valid`
          (`AbilitySystemComponent.TargetConfirm` (`AbilitySystemBlueprintLibrary.GetAbilitySystemComponent` _controlledunit))
          (set `self.Targeting` false)
          (`KismetSystemLibrary.PrintString` "target confirm")))
      (else
        (`self.SelectHero`)))))

(event `InputAction|UseAbility1`
  (params (Key :type "Key Structure"))
  (:`Pressed`
    (`self.SpellAttack` 1)))

(event `InputAction|UseAbility2`
  (params (Key :type "Key Structure"))
  (:`Pressed`
    (`self.SpellAttack` 2)))

(event `InputAction|UseAbility3`
  (params (Key :type "Key Structure"))
  (:`Pressed`
    (`self.SpellAttack` 3)))

(event `InputAction|CancelTargetting`
  (params (Key :type "Key Structure"))
  (bind _controlledunit (`self.ControlledUnit`))
  (:`Pressed`
    (`/Engine/EditorBlueprintResources/StandardMacros.IsValid` _controlledunit
      (:`Is Valid`
        (`AbilitySystemComponent.TargetCancel` (`AbilitySystemBlueprintLibrary.GetAbilitySystemComponent` _controlledunit))
        (set `self.Targeting` false)))))

(event `InputAction|UseAbility4`
  (params (Key :type "Key Structure"))
  (:`Pressed`
    (`self.SpellAttack` 4)))

(event `InputAction|UseAbility5`
  (params (Key :type "Key Structure"))
  (:`Pressed`
    (`self.SpellAttack` 5)))

(event `InputAction|Stop`
  (params (Key :type "Key Structure"))
  (bind _controlledunit (`self.ControlledUnit`))
  (:`Pressed`
    (`/Engine/EditorBlueprintResources/StandardMacros.IsValid` _controlledunit
      (:`Is Valid`
        (`AP_Hero.CancelAllAttack` _controlledunit)))))

(event `InputAction|UseAbility6`
  (params (Key :type "Key Structure"))
  (:`Pressed`
    (`self.SpellAttack` 6)))

(fn `SelectHero`
  (bind (_worldlocation _worlddirection) (`self.DeprojectMousePositionToWorld`))
  (bind _controlledunit (`self.ControlledUnit`))
  (`/Engine/EditorBlueprintResources/StandardMacros.IsValid` _controlledunit
    (:`Is Valid`
      (`AP_Hero.SelectHero` _controlledunit false))
    (:`Is Not Valid`
      _))
  (bind _outhit (`KismetSystemLibrary.LineTraceSingle` _worldlocation (+ _worldlocation (* _worlddirection 20000.0)) "TraceTypeQuery7" false (`|MakeArray` (`self.ControlledUnit`) :!type "Actor Object Reference")))
  (bind _asap_hero (cast `AP_Hero` (`.HitActor` (`GameplayStatics.BreakHitResult` _outhit)))
    (:`then`
      (bind _output_get (set `self.ControlledUnit` _asap_hero))
      (`AP_Hero.SelectHero` _output_get true)
      (`self.OnControlledUnitChanged` _output_get))
    (:`CastFailed`
      (`AP_Hero.SelectHero` (`self.ControlledUnit`) true))))

(fn `SpellAttack`
  (params (AbilitySlot :type Integer))
  (bind _controlledunit (`self.ControlledUnit`))
  (`/Engine/EditorBlueprintResources/StandardMacros.IsValid` _controlledunit
    (:`Is Valid`
      (`AP_Hero.SpellAttack` _controlledunit AbilitySlot)
      (set `self.Targeting` (`AP_Hero.IsTargeting` _controlledunit)))))

(fn `UserConstructionScript`)
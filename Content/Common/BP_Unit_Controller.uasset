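; Player controller for RTS/MOBA-style hero control: pans the camera pawn, selects a hero by click and issues move, attack, ability, stop and hold orders.
; Ability keys enter crosshair targeting for unit- or ground-target skills and cast others immediately.
; Orders mostly write target, range, skill slot and state to the hero's AI Blackboard.
; Ability inputs set TargetingAbility after EnterTargeting runs, so it checks the previous slot.
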(event `InputAxis|CameraX`
  (params (AxisValue :type "Float (single-precision)"))
  (bind _returnvalue (`self.K2_GetPawn`))
  (`Pawn.AddMovementInput` _returnvalue (`SceneComponent.GetRightVector` (`Actor.RootComponent` _returnvalue)) AxisValue false))

(event `self.ReceiveBeginPlay`)

(event `InputAxis|CameraY`
  (params (AxisValue :type "Float (single-precision)"))
  (bind _returnvalue (`self.K2_GetPawn`))
  (`Pawn.AddMovementInput` _returnvalue (`SceneComponent.GetForwardVector` (`Actor.RootComponent` _returnvalue)) AxisValue false))

(event `Key|RightMouseButton`
  (params (Key :type "Key Structure"))
  (:`Pressed`
    (if (`self.Targeting`)
      (`self.CancelTargeting`)
      (else
        (`self.Move`)))))

(event `Key|LeftMouseButton`
  (params (Key :type "Key Structure"))
  (:`Pressed`
    (if (`self.Targeting`)
      (`self.ConfirmTargeting`)
      (else
        (`self.SelectHero`)))))

(event `InputAction|WeaponAbility`
  (params (Key :type "Key Structure"))
  (:`Pressed`
    (`self.EnterTargeting`)
    (set `self.TargetingAbility` 0)))

(event `InputAction|UseAbility1`
  (params (Key :type "Key Structure"))
  (:`Pressed`
    (`self.EnterTargeting`)
    (set `self.TargetingAbility` 1)))

(event `InputAction|UseAbility2`
  (params (Key :type "Key Structure"))
  (:`Pressed`
    (`self.EnterTargeting`)
    (set `self.TargetingAbility` 2)))

(event `Key|M`
  (params (Key :type "Key Structure"))
  (:`Released`
    (`KismetSystemLibrary.PrintString` "M pressed")
    (bind _asac_basic (cast `/Game/Common/AI/AC_Basic` (`AIBlueprintHelperLibrary.GetAIController` (`self.ControlledUnit`))))
    (`/Game/Common/AI/AC_Basic.AttackMove` _asac_basic (`.Location` (`GameplayStatics.BreakHitResult` (`self.GetHitResultUnderCursorByChannel` "TraceTypeQuery3" false))))))

(event `InputAction|UseAbility3`
  (params (Key :type "Key Structure"))
  (:`Pressed`
    (`self.EnterTargeting`)
    (set `self.TargetingAbility` 3)))

(event `InputAction|UseAbility4`
  (params (Key :type "Key Structure"))
  (:`Pressed`
    (`self.EnterTargeting`)
    (set `self.TargetingAbility` 4)))

(event `Key|H`
  (params (Key :type "Key Structure"))
  (:`Pressed`
    (`self.Hold`)))

(event `Key|S`
  (params (Key :type "Key Structure"))
  (:`Pressed`
    (`self.Stop`)))

(fn `CancelTargeting`
  (set `self.Targeting` false)
  (set `self.CurrentMouseCursor` "Default"))

(fn `ClearTargetInfo`
  (bind _returnvalue (`AIBlueprintHelperLibrary.GetBlackboard` (`self.ControlledUnit`)))
  (`BlackboardComponent.SetValueAsInt` _returnvalue (`self.SkillToCast_KeyName`) -1)
  (`BlackboardComponent.ClearValue` _returnvalue (`self.TargetActor_KeyName`))
  (`BlackboardComponent.SetValueAsFloat` _returnvalue (`self.CastRange_KeyName`) 99999.0)
  (`BlackboardComponent.ClearValue` _returnvalue (`self.TargetLocation_KeyName`)))

(fn `ConfirmTargeting`
  (locals (IsUnitTarget :type Boolean) (IsGroundTarget :type Boolean) (IsBasicAttack :type Boolean))
  (bind (_hitresult _returnvalue) (`self.GetHitResultUnderCursorByChannel` "TraceTypeQuery3" false))
  (bind (_hitresult_2 _returnvalue_2) (`self.GetHitResultUnderCursorByChannel` "TraceTypeQuery3" false))
  (bind (_hitresult_3 _returnvalue_3) (`self.GetHitResultUnderCursorByChannel` "TraceTypeQuery7" false))
  (`self.ClearTargetInfo`)
  (set `local.IsBasicAttack` (== (`self.TargetingAbility`) 0))
  (bind _result (`self.GetAbilityInfo` (`self.TargetingAbility`)))
  (bind _returnvalue_4 (`GameplayStatics.GetObjectClass` _result))
  (set `local.IsUnitTarget` (`KismetMathLibrary.ClassIsChildOf` _returnvalue_4 "/Game/AgeOfDualBlade/Abilities/Core/Base/Unit_Target_Skill.Unit_Target_Skill_C"))
  (set `local.IsGroundTarget` (`KismetMathLibrary.ClassIsChildOf` _returnvalue_4 "/Game/AgeOfDualBlade/Abilities/Core/Base/Ground_Target_Skill.Ground_Target_Skill_C"))
  (if (`local.IsUnitTarget`)
    (if _returnvalue_3
      (`self.WriteActorTarget` (`.HitActor` (`GameplayStatics.BreakHitResult` _hitresult_3)))
      (bind _asunit_target_skill (cast `/Game/AgeOfDualBlade/Abilities/Core/Base/Unit_Target_Skill` _result)
        (:`then`
          (`self.WriteSkillToCast` (`self.TargetingAbility`))
          (`self.WriteCastRange` (`/Game/AgeOfDualBlade/Abilities/Core/Base/Unit_Target_Skill.Range` _asunit_target_skill)))
        (:`CastFailed`
          _))
      (`self.WriteState` (select `bool` (`local.IsBasicAttack`) :`false` "NewEnumerator0" :`true` "NewEnumerator7" :!type "/Game/Common/AI/AI_State Enum"))
      (set `self.Targeting` false)
      (set `self.CurrentMouseCursor` "Default")
      (elif (`local.IsBasicAttack`)
        (if _returnvalue_2
          (`self.WriteActorTarget` null)
          (`self.WriteLocationTarget` (`.Location` (`GameplayStatics.BreakHitResult` _hitresult_2)))
          (bind _asunit_target_skill_2 (cast `/Game/AgeOfDualBlade/Abilities/Core/Base/Unit_Target_Skill` _result)
            (:`then`
              (`self.WriteSkillToCast` (`self.TargetingAbility`))
              (`self.WriteCastRange` (`/Game/AgeOfDualBlade/Abilities/Core/Base/Unit_Target_Skill.Range` _asunit_target_skill_2)))
            (:`CastFailed`
              _))
          (`self.WriteState` "NewEnumerator6")
          (set `self.Targeting` false)
          (set `self.CurrentMouseCursor` "Default"))))
    (elif (`local.IsGroundTarget`)
      (if _returnvalue
        (`self.WriteActorTarget` null)
        (bind _asground_target_skill (cast `/Game/AgeOfDualBlade/Abilities/Core/Base/Ground_Target_Skill` _result)
          (:`then`
            (`self.WriteCastRange` (`/Game/AgeOfDualBlade/Abilities/Core/Base/Ground_Target_Skill.Range` _asground_target_skill))
            (`self.WriteSkillToCast` (`self.TargetingAbility`)))
          (:`CastFailed`
            _))
        (`self.WriteLocationTarget` (`.Location` (`GameplayStatics.BreakHitResult` _hitresult)))
        (`self.WriteState` "NewEnumerator3")
        (set `self.Targeting` false)
        (set `self.CurrentMouseCursor` "Default"))
      (else
        (`self.WriteCastRange` 0.0)))))

(fn `EnterTargeting`
  (locals (IsGroundTarget :type Boolean) (IsUnitTarget :type Boolean))
  (bind _result (`self.GetAbilityInfo` (`self.TargetingAbility`)))
  (bind _returnvalue (`GameplayStatics.GetObjectClass` _result))
  (set `local.IsUnitTarget` (`KismetMathLibrary.ClassIsChildOf` _returnvalue "/Game/AgeOfDualBlade/Abilities/Core/Base/Unit_Target_Skill.Unit_Target_Skill_C"))
  (set `local.IsGroundTarget` (`KismetMathLibrary.ClassIsChildOf` _returnvalue "/Game/AgeOfDualBlade/Abilities/Core/Base/Ground_Target_Skill.Ground_Target_Skill_C"))
  (if (or (`local.IsUnitTarget`) (`local.IsGroundTarget`))
    (set `self.CurrentMouseCursor` "Crosshairs")
    (set `self.Targeting` true)
    (else
      (`KismetSystemLibrary.PrintString` (`KismetStringLibrary.Concat_StrStr` "this skill is, " (`KismetSystemLibrary.GetClassDisplayName` (`GameplayStatics.GetObjectClass` _result)) ", not unit target, not ground target, so skip targeting phase" (`KismetStringLibrary.Conv_IntToString` (`self.TargetingAbility`))))
      (`AP_Hero.SpellAttack` (`self.ControlledUnit`) (`self.TargetingAbility`)))))

(fn `GetAbilityInfo`
  (params (Index :type Integer))
  (returns (Result :type "GameplayAbility Object Reference"))
  (bind _returnvalue (`AP_Hero.GetSpell` (`self.ControlledUnit`) Index))
  (`/Engine/EditorBlueprintResources/StandardMacros.IsValid` _returnvalue
    (:`Is Valid`
      (return _returnvalue))
    (:`Is Not Valid`
      (return _returnvalue))))

(fn `Hold`
  (`self.ClearTargetInfo`)
  (`BlackboardComponent.SetValueAsEnum` (`AIBlueprintHelperLibrary.GetBlackboard` (`self.ControlledUnit`)) (`self.AIState_KeyName`) (enumliteral `/Game/Common/AI/AI_State` "NewEnumerator1")))

(fn `Move`
  (bind (_hitresult _returnvalue) (`self.GetHitResultUnderCursorByChannel` "TraceTypeQuery3" false))
  (bind _controlledunit (`self.ControlledUnit`))
  (bind (_bblockinghit _binitialoverlap _time _distance _location) (`GameplayStatics.BreakHitResult` _hitresult))
  (`self.ClearTargetInfo`)
  (`/Engine/EditorBlueprintResources/StandardMacros.IsValid` _controlledunit
    (:`Is Valid`
      (if _returnvalue
        (`Character.StopAnimMontage` _controlledunit null)
        (`GameplayStatics.SpawnEmitterAtLocation` "/Game/LinhiBlade/MouseClickParticle/P_MouseClick.P_MouseClick" _location (struct :`Roll` 90.0) (1.0 1.0 1.0) true "AutoRelease")
        (`self.WriteActorTarget` null)
        (`self.WriteLocationTarget` _location)
        (`self.WriteState` "NewEnumerator5")))))

(fn `SelectHero`
  (bind (_worldlocation _worlddirection) (`self.DeprojectMousePositionToWorld`))
  (bind _controlledunit (`self.ControlledUnit`))
  (set `self.Targeting` false)
  (`/Engine/EditorBlueprintResources/StandardMacros.IsValid` _controlledunit
    (:`Is Valid`
      (`AP_Hero.SelectHero` _controlledunit false))
    (:`Is Not Valid`
      _))
  (bind _outhit (`KismetSystemLibrary.LineTraceSingle` _worldlocation (+ _worldlocation (* _worlddirection 20000.0)) "TraceTypeQuery7" false (`|MakeArray` (`self.ControlledUnit`) :!type "Actor Object Reference")))
  (bind _asap_hero (cast `AP_Hero` (`.HitActor` (`GameplayStatics.BreakHitResult` _outhit)))
    (:`then`
      (bind _output_get (set `self.ControlledUnit` _asap_hero))
      (`AP_Hero.SelectHero` _output_get true)
      (`self.OnControlledUnitChanged` _output_get))
    (:`CastFailed`
      (`AP_Hero.SelectHero` (`self.ControlledUnit`) true))))

(fn `Stop`
  (`self.ClearTargetInfo`)
  (`BlackboardComponent.SetValueAsEnum` (`AIBlueprintHelperLibrary.GetBlackboard` (`self.ControlledUnit`)) (`self.AIState_KeyName`) (enumliteral `/Game/Common/AI/AI_State` "NewEnumerator1")))

(fn `UserConstructionScript`)

(fn `WriteActorTarget`
  (params (TargetActor :type "Actor Object Reference"))
  (bind _targetactor_keyname (`self.TargetActor_KeyName`))
  (bind _returnvalue (`AIBlueprintHelperLibrary.GetBlackboard` (`self.ControlledUnit`)))
  (`/Engine/EditorBlueprintResources/StandardMacros.IsValid` TargetActor
    (:`Is Valid`
      (`BlackboardComponent.SetValueAsObject` _returnvalue _targetactor_keyname TargetActor))
    (:`Is Not Valid`
      (`BlackboardComponent.ClearValue` _returnvalue _targetactor_keyname))))

(fn `WriteCastRange`
  (params (Range :type "Float (double-precision)"))
  (`BlackboardComponent.SetValueAsFloat` (`AIBlueprintHelperLibrary.GetBlackboard` (`self.ControlledUnit`)) (`self.CastRange_KeyName`) Range))

(fn `WriteLocationTarget`
  (params (TargetLocation :type "Vector Structure"))
  (`BlackboardComponent.SetValueAsVector` (`AIBlueprintHelperLibrary.GetBlackboard` (`self.ControlledUnit`)) (`self.TargetLocation_KeyName`) TargetLocation))

(fn `WriteSkillToCast`
  (params (Slot :type Integer))
  (`BlackboardComponent.SetValueAsInt` (`AIBlueprintHelperLibrary.GetBlackboard` (`self.ControlledUnit`)) (`self.SkillToCast_KeyName`) Slot))

(fn `WriteState`
  (params (State :type "/Game/Common/AI/AI_State Enum" :default "NewEnumerator0"))
  (`BlackboardComponent.SetValueAsEnum` (`AIBlueprintHelperLibrary.GetBlackboard` (`self.ControlledUnit`)) (`self.AIState_KeyName`) State))
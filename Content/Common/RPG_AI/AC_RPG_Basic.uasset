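; AC_RPG_Basic is a basic AI controller that starts the RPG master behavior tree on BeginPlay, then resets the blackboard's ability, state and cast range keys.
; Helper functions get and set the blackboard target actor, pick a random perceived actor, and check whether an actor is currently perceived by sight.
; Retargeting logic for lost targets exists but is unconnected, and the perception update event is empty.
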(event `self.ReceiveBeginPlay`
  (`self.RunBehaviorTree` "/Game/Common/RPG_AI/BT_RPG_Master.BT_RPG_Master")
  (`self.ResetBB`))

(event `self.AIPerception.OnPerceptionUpdated`
  (params (UpdatedActors :type "Array of Actor Object Reference (by ref)")))

(fn `GetCurrentTarget`
  (returns (Result :type "Actor Object Reference"))
  (bind _asactor (cast `Actor` (`BlackboardComponent.GetValueAsObject` (`AIBlueprintHelperLibrary.GetBlackboard` (`self.K2_GetPawn`)) (`self.TargetActor_KeyName`)))
    (:`then`
      (return _asactor))
    (:`CastFailed`
      (return null))))

(fn `GetRandomTarget`
  (returns (Result :type "Actor Object Reference"))
  (bind _outactors (`AIPerceptionComponent.GetPerceivedActors` (`self.AIPerception`) null))
  (bind _returnvalue (`KismetArrayLibrary.Array_Length` _outactors))
  (if (> _returnvalue 0)
    (return (`|GetArrayItem` _outactors (`KismetMathLibrary.RandomInteger` _returnvalue)))
    (else
      (return null))))

(fn `IsInPerceivedList`
  (params (ItemToFind :type "Actor Object Reference (by ref)"))
  (returns (ReturnValue :type Boolean))
  (return (>= (`KismetArrayLibrary.Array_Find` (`AIPerceptionComponent.GetCurrentlyPerceivedActors` (`self.AIPerception`) "/Script/AIModule.AISense_Sight") ItemToFind) 0)))

(fn `ResetBB`
  (bind _returnvalue (`AIBlueprintHelperLibrary.GetBlackboard` (`self.K2_GetPawn`)))
  (`BlackboardComponent.SetValueAsInt` _returnvalue (`self.AbilityToCast_KeyName`) -1)
  (`BlackboardComponent.SetValueAsEnum` _returnvalue (`self.CurrentState_KeyName`) (enumliteral `/Game/Common/RPG_AI/AI_BasicState` "NewEnumerator0"))
  (`BlackboardComponent.SetValueAsFloat` _returnvalue (`self.CastRange_KeyName`) 100000.0))

(fn `SetCurrentTarget`
  (params (NewTarget :type "Actor Object Reference"))
  (`BlackboardComponent.SetValueAsObject` (`AIBlueprintHelperLibrary.GetBlackboard` (`self.K2_GetPawn`)) (`self.TargetActor_KeyName`) NewTarget))

(fn `UserConstructionScript`)